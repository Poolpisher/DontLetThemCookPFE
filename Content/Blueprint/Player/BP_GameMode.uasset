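; Game mode Blueprint that stores the latest checkpoint and returns the player to it.
; UpdateCheckpoint records a checkpoint's position, rotation and map name.
; LoadCheckpoint ends active dialogue, shows a loading screen, restores game input and player state, then teleports the player and minions after a short delay.
; It later clears the queryable IsCheckpointLoad flag; level-streaming reload logic is present but disconnected.
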(event EventLoadCheckpoint
  (bind _returnvalue (Game|GetPlayerController 0))
  ;[1 0.3333 0 1 34] Load level
  (bind _asbp_player (Utilities|Casting|CastToBP_Player (Game|Player|GetPlayerPawn 0)))
  (Variables|Default|SetPlayerRef _asbp_player)
  (bind _currentdialogue (Variables|/Game/Blueprint/Player/BP_Player.BP_Player_C|GetcurrentDialogue (Variables|Default|GetPlayerRef))
    (:then
      (Default|ForceFinishDialogue _currentdialogue))
    (:else
      _))
  (bind _returnvalue_2 (UserInterface|CreateWidget "/Game/1_UI/3_Widgets/Loading/W_LoadingScreen.W_LoadingScreen_C"))
  (bind _output_get (Variables|Default|SetloadingScreen _returnvalue_2))
  (UserInterface|Viewport|AddtoViewport _output_get 0)
  (Utilities|FlowControl|Delay 1.0)
  (Default|FinishLoad (Variables|Default|GetloadingScreen))
  (Input|SetInputModeGameOnly _returnvalue true)
  (Variables|/Script/Engine.PlayerController|SetbShowMouseCursor _returnvalue false)
  (Default|CloseCheat (Variables|Default|GetPlayerRef))
  (Default|SetCam (Variables|/Game/Blueprint/Player/BP_Player.BP_Player_C|Getcamera (Variables|Default|GetPlayerRef)))
  (Default|ExitRopeMapLoad (Variables|Default|GetPlayerRef))
  (Transformation|SetActorLocationAndRotation (Variables|Default|GetPlayerRef) (Variables|Default|GetCheckpointPosition) (Variables|Default|GetCheckpointRotation) false true)
  (Default|TPMinions (Variables|Default|GetPlayerRef))
  (Utilities|FlowControl|Delay 2.5)
  (Variables|Default|SetIsCheckpointLoad false))

(event EventUpdateCheckpoint
  (params (CheckpointRef :type Actor%20Object%20Reference) (CheckpointMap :type Name :default "None"))
  (bind _returnvalue (Transformation|GetActorTransform CheckpointRef))
  (Variables|Default|SetCheckpointPosition (.location _returnvalue))
  (Variables|Default|SetCheckpointRotation (.rotation _returnvalue))
  (Variables|Default|SetCheckpointMap CheckpointMap))

(fn ConstructionScript)

(fn CheckIsCheckpointLoad
  (return (Variables|Default|GetIsCheckpointLoad)))