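; Dialogue component that plays an NPC's conversation from a data table, with gift-giving reactions.
; SpawnDialogue shows the current row in the player's dialogue widget, triggers the NPC reaction, and, only for rows with sound, plays it and toggles the gift menu.
; Finishing advances rows unless the menu blocks it; the end restores the first table, game input and briefly disables jumping.
; GiveItem finds the character's item reaction in TableReact and closes the menu.
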(event Custom|SpawnDialogue
  (bind _returnvalue (Game|GetPlayerCharacter 0))
  (bind _dialogue (Variables|Default|Getdialogue))
  (bind _asbp_player (Utilities|Casting|CastToBP_Player _returnvalue))
  ;[0 0 1 1 34] Comment
  (Input|SetInputModeUIOnly (Game|GetPlayerController 0) 0 "DoNotLock" true)
  (Utilities|FlowControl|DoOnce false
    (:Completed
      (bind _returnvalue_2 (UserInterface|CreateWidget "/Game/Widgets/Dialogue/W_Dialogue.W_Dialogue_C" 0 self))
      (bind _output_get (Variables|/Game/Blueprint/Player/BP_Player.BP_Player_C|SetcurrentDialogue _asbp_player _returnvalue_2))
      (UserInterface|Viewport|AddtoViewport _output_get 0)
      (bind _outrownames (DataTable|GetDataTableRowNames _dialogue))
      (bind _returnvalue_3 (Utilities|GetDataTableRow _dialogue (Utilities|Array|Get(acopy) _outrownames (Variables|Default|Getindex)))
        (:then
          (bind _asbp_npc (Utilities|Casting|CastToBP_NPC (Components|GetOwner))
            (:then
              (Default|PlayReact _asbp_npc (.react (Utilities|Struct|BreakStruct_Dialogue _returnvalue_3))))
            (:CastFailed
              _))
          (Default|WriteText (Variables|/Game/Blueprint/Player/BP_Player.BP_Player_C|GetcurrentDialogue _asbp_player) (Utilities|Text|ToText(String) (Utilities|String|EnumtoString (.Name (Utilities|Struct|BreakStruct_Dialogue _returnvalue_3)))) (.Dialogue (Utilities|Struct|BreakStruct_Dialogue _returnvalue_3)) (.nextDialogues (Utilities|Struct|BreakStruct_Dialogue _returnvalue_3)))
          (Utilities|IsValid (.sound (Utilities|Struct|BreakStruct_Dialogue _returnvalue_3))
            (:Is%20Valid
              (Audio|SpawnSound2D (.sound (Utilities|Struct|BreakStruct_Dialogue _returnvalue_3)) 1.0 1.0 0.0 0)
              (if (.openGiftMenu (Utilities|Struct|BreakStruct_Dialogue _returnvalue_3))
                (bind _returnvalue_4 (UserInterface|CreateWidget "/Game/Widgets/Dialogue/W_GiftMenu.W_GiftMenu_C" 0 self))
                (bind _output_get_2 (Variables|Default|SetgiftMenu _returnvalue_4))
                (UserInterface|Viewport|AddtoViewport _output_get_2 0)
                (else
                  (bind _giftmenu (Variables|Default|GetgiftMenu)
                    (:then
                      (Widget|RemovefromParent _giftmenu)
                      (Variables|Default|SetgiftMenu 0)
                      (Variables|/Script/Engine.PlayerController|SetbShowMouseCursor (Game|GetPlayerController 0) false))
                    (:else)))))))))))

(event Custom|OnFinishDialogue
  (params (forceNextDialogue :type Boolean))
  (bind _returnvalue (Game|GetPlayerCharacter 0))
  (bind _asbp_player (Utilities|Casting|CastToBP_Player _returnvalue))
  ;[0 0 1 1 34] Comment
  (if forceNextDialogue
    _
    (else
      (Variables|Default|GetgiftMenu
        (:then)
        (:else
          _))))
  (bind _result (Math|Integer|IncrementInt (Variables|Default|Getindex))
    (:%20%20
      (bind _outrownames (DataTable|GetDataTableRowNames (Variables|Default|Getdialogue)))
      (if (>= _result (Utilities|Array|Length _outrownames))
        (Variables|Default|Setindex 0)
        (Widget|RemovefromParent (Variables|/Game/Blueprint/Player/BP_Player.BP_Player_C|GetcurrentDialogue (.AsBP%20Player (Utilities|Casting|CastToBP_Player (Game|GetPlayerCharacter 0)))))
        (Input|SetInputModeGameOnly (Game|GetPlayerController 0) true)
        (CallFunction|LockJump)
        (Variables|Default|Setdialogue (Variables|Default|GetfirstDialogue))
        (Utilities|FlowControl|DoOnce false) ; enters at Reset
        (else
          (Widget|RemovefromParent (Variables|/Game/Blueprint/Player/BP_Player.BP_Player_C|GetcurrentDialogue (.AsBP%20Player (Utilities|Casting|CastToBP_Player (Game|GetPlayerCharacter 0)))))
          (Utilities|FlowControl|Sequence
            (:then_0
              (Utilities|FlowControl|DoOnce false) ; enters at Reset
            )
            (:then_1
              (CallFunction|SpawnDialogue))))))))

(event Custom|LockJump
  (bind _returnvalue (Game|GetPlayerCharacter 0))
  (bind _asbp_player (Utilities|Casting|CastToBP_Player _returnvalue))
  (bind _charactermovement (Variables|/Script/Engine.Character|GetCharacterMovement _asbp_player))
  ;[0 1 0 1 34] Jump lock
  (bind _output_get (Variables|Default|SetJump%20Z%20Velocity (Variables|/Script/Engine.CharacterMovementComponent|GetJumpZVelocity _charactermovement)))
  (Variables|/Script/Engine.CharacterMovementComponent|SetJumpZVelocity _charactermovement 0.0)
  (Utilities|FlowControl|Delay 0.5)
  (Variables|/Script/Engine.CharacterMovementComponent|SetJumpZVelocity _charactermovement _output_get))

(event Custom|ForceNextLine
  (bind _returnvalue (Game|GetPlayerCharacter 0))
  (bind _dialogue (Variables|Default|Getdialogue))
  (bind _asbp_player (Utilities|Casting|CastToBP_Player _returnvalue))
  ;[0 0 1 1 34] Comment
  (Widget|RemovefromParent (Variables|/Game/Blueprint/Player/BP_Player.BP_Player_C|GetcurrentDialogue (.AsBP%20Player (Utilities|Casting|CastToBP_Player (Game|GetPlayerCharacter 0)))))
  (Utilities|FlowControl|Sequence
    (:then_0
      (Utilities|FlowControl|DoOnce false) ; enters at Reset
    )
    (:then_1
      (CallFunction|SpawnDialogue))))

(event Custom|GiveItem
  (params (item :type Enum_Items%20Enum :default "NewEnumerator0"))
  (bind _tablereact (Variables|Default|GettableReact))
  ;[0 0.15 0.125 1 34] Give item
  (bind _outrownames (DataTable|GetDataTableRowNames _tablereact))
  (bind _array_element (Utilities|Array|ForEachLoopwithBreak _outrownames :!label _label)
    (:LoopBody
      (bind _returnvalue (Utilities|GetDataTableRow _tablereact _array_element)
        (:then
          (if (Utilities|Enum|Equal(Enum) (.character (Utilities|Struct|BreakStruct_React _returnvalue)) (Variables|Default|Getcharacters))
            (bind _array_element_2 (Utilities|Array|ForEachLoopwithBreak (.reactions (Utilities|Struct|BreakStruct_React _returnvalue)) :!label _label_2)
              (:LoopBody
                (bind _asbp_player (Utilities|Casting|CastToBP_Player (Game|GetPlayerCharacter 0)))
                (if (Utilities|Enum|Equal(Enum) (.item (Utilities|Struct|BreakStruct_ItemReact _array_element_2)) item)
                  (Default|WriteText (Variables|/Game/Blueprint/Player/BP_Player.BP_Player_C|GetcurrentDialogue _asbp_player) (Utilities|Text|ToText(String) (Utilities|String|EnumtoString (Variables|Default|Getcharacters))) (.line (Utilities|Struct|BreakStruct_ItemReact _array_element_2)))
                  (bind _asbp_npc (Utilities|Casting|CastToBP_NPC (Components|GetOwner))
                    (:then
                      (Default|PlayReact _asbp_npc (.reactions (Utilities|Struct|BreakStruct_ItemReact _array_element_2))))
                    (:CastFailed
                      _))
                  (bind _giftmenu (Variables|Default|GetgiftMenu)
                    (:then
                      (Widget|RemovefromParent _giftmenu)
                      (Variables|Default|SetgiftMenu 0)
                      (Variables|/Script/Engine.PlayerController|SetbShowMouseCursor (Game|GetPlayerController 0) false))
                    (:else
                      _))
                  (Utilities|FlowControl|Sequence
                    (:then_0
                      (goto _label Break))
                    (:then_1
                      (goto _label_2 Break))))))))))))

(event EventBeginPlay
  ;[0 0 0 1 34] Start
  (Variables|Default|SetfirstDialogue (Variables|Default|Getdialogue)))