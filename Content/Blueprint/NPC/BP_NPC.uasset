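; BP_NPC is a non-player character that the player can interact with to spawn dialogue through BPCDialogue.
; One collider shows and animates the interact widget for BP_Player, while a second toggles a bark TextRender on overlap.
; Interacting hides or destroys the prompt depending on InteractionType, then spawns dialogue and hides the bark.
; PlayReact swaps the Niagara asset and offset by reaction type to show emotes.
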(event OnComponentBeginOverlap(Collider)
  (params (OverlappedComponent :type Primitive%20Component%20Object%20Reference) (OtherActor :type Actor%20Object%20Reference) (OtherComp :type Primitive%20Component%20Object%20Reference) (OtherBodyIndex :type Integer) (bFromSweep :type Boolean) (SweepResult :type Hit%20Result%20Structure%20%28by%20ref%29))
  (bind _widget (Variables|Default|GetWidget))
  ;[0 1 1 1 34] Widget interact
  (Utilities|Casting|CastToBP_Player OtherActor)
  (Development|SetHiddeninGame _widget false false)
  (bind _asw_interact (Utilities|Casting|CastToW_Interact (UserInterface|GetWidget _widget)))
  (Default|PlayAnim _asw_interact))

(event OnComponentEndOverlap(Collider)
  (params (OverlappedComponent :type Primitive%20Component%20Object%20Reference) (OtherActor :type Actor%20Object%20Reference) (OtherComp :type Primitive%20Component%20Object%20Reference) (OtherBodyIndex :type Integer))
  ;[0 1 1 1 34] Widget interact
  (Utilities|Casting|CastToBP_Player OtherActor)
  (Development|SetHiddeninGame (Variables|Default|GetWidget) true false))

(event OnComponentBeginOverlap(ColliderBark)
  (params (OverlappedComponent :type Primitive%20Component%20Object%20Reference) (OtherActor :type Actor%20Object%20Reference) (OtherComp :type Primitive%20Component%20Object%20Reference) (OtherBodyIndex :type Integer) (bFromSweep :type Boolean) (SweepResult :type Hit%20Result%20Structure%20%28by%20ref%29))
  (Utilities|Casting|CastToBP_Player OtherActor)
  (Rendering|SetVisibility (Variables|Default|GetTextRender) true false))

(event OnComponentEndOverlap(ColliderBark)
  (params (OverlappedComponent :type Primitive%20Component%20Object%20Reference) (OtherActor :type Actor%20Object%20Reference) (OtherComp :type Primitive%20Component%20Object%20Reference) (OtherBodyIndex :type Integer))
  (Utilities|Casting|CastToBP_Player OtherActor)
  (Rendering|SetVisibility (Variables|Default|GetTextRender) false false))

(event Custom|PlayReact
  (params (reacts :type Enum_Reactions%20Enum :default "NewEnumerator7"))
  (bind _niagarareact (Variables|Default|GetNiagaraReact))
  ;[0 0.1559 0.1299 1 34] Reactions
  (Class|NiagaraComponent|SetAsset (Variables|Default|GetNiagaraReact) (Utilities|Select :Index reacts :NewEnumerator8 0 :NewEnumerator7 "/Game/Maps/GA/VFX/dialogue_reactions/ankward/N_goutte.N_goutte" :NewEnumerator9 "/Game/Maps/GA/VFX/dialogue_reactions/happy/N_happy.N_happy" :NewEnumerator10 "/Game/Maps/GA/VFX/dialogue_reactions/surprise/N_surprise.N_surprise" :NewEnumerator11 "/Game/Maps/GA/VFX/dialogue_reactions/surprise/N_surprise.N_surprise") false)
  (if (Utilities|Enum|NotEqual(Enum) reacts "NewEnumerator8")
    (Transformation|SetRelativeLocation _niagarareact (Utilities|Select :Index reacts :NewEnumerator8 "30.000000,0.000000,60.000000" :NewEnumerator7 "40.000000,20.000000,60.000000" :NewEnumerator9 "30.000000,0.000000,60.000000" :NewEnumerator10 "0, 0, 0" :NewEnumerator11 "30.000000,0.000000,60.000000") false false)
    (Components|Activation|Activate _niagarareact true)))

(event EventSelect)

(event EventDeselect)

(event EventBeginPlay
  (Rendering|SetVisibility (Variables|Default|GetTextRender) false false))

(event EventInteract
  (params (Interactor :type BPC%20Interactor%20Object%20Reference))
  (switch Utilities|FlowControl|Switch|SwitchonEnum_InteractionType (Variables|Default|GetinteractionType)
    (:NewEnumerator0
      (Development|SetHiddeninGame (Variables|Default|GetWidget) true false :!label _label))
    (:NewEnumerator1
      (Utilities|FlowControl|DoOnce false
        (:Completed
          (Components|DestroyComponent (Variables|Default|GetWidget)))))
    (:NewEnumerator2
      (goto _label)))
  (Default|SpawnDialogue (Variables|Default|GetBPC_Dialogue))
  (Rendering|SetVisibility (Variables|Default|GetTextRender) false false))

(fn ConstructionScript)