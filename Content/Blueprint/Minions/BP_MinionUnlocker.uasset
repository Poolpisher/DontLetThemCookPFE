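; BP_MinionUnlocker is a placeable actor that unlocks a chosen minion, Karl (toad) or Betty (beetle), as soon as it begins play.
; If that minion class is missing from the GI_Instance Minions list, it adds it and calls SetMinions on the player.
; The construction script sets the billboard sprite to the icon of the selected minion.
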(event EventBeginPlay
  (bind _asgi_instance (Utilities|Casting|CastToGI_Instance (Game|GetGameInstance)))
  (if (not (Utilities|Select :Index (Variables|Default|GetminionsToUnlock) :NewEnumerator0 (Utilities|Array|ContainsItem (Variables|/Game/Blueprint/GI_Instance.GI_Instance_C|Getminions _asgi_instance) "/Game/Blueprint/Minions/BP_MinionToad.BP_MinionToad_C") :NewEnumerator1 (Utilities|Array|ContainsItem (Variables|/Game/Blueprint/GI_Instance.GI_Instance_C|Getminions _asgi_instance) "/Game/Blueprint/Minions/BP_MinionBeetle.BP_MinionBeetle_C")))
    (switch Utilities|FlowControl|Switch|SwitchonEnum_Minions (Variables|Default|GetminionsToUnlock)
      (:NewEnumerator0
        (Utilities|Array|AddUnique (Variables|/Game/Blueprint/GI_Instance.GI_Instance_C|Getminions _asgi_instance) "/Game/Blueprint/Minions/BP_MinionToad.BP_MinionToad_C"))
      (:NewEnumerator1
        (Utilities|Array|AddUnique (Variables|/Game/Blueprint/GI_Instance.GI_Instance_C|Getminions _asgi_instance) "/Game/Blueprint/Minions/BP_MinionBeetle.BP_MinionBeetle_C")))
    (bind _asbp_player (Utilities|Casting|CastToBP_Player (Game|GetPlayerCharacter 0)))
    (Default|SetMinions _asbp_player)))

(fn ConstructionScript
  (Rendering|Components|Sprite|SetSprite (Variables|Default|GetBillboard) (Utilities|Select :Index (Variables|Default|GetminionsToUnlock) :NewEnumerator0 "/Game/1_UI/1_Textures/T_Icon_Karl.T_Icon_Karl" :NewEnumerator1 "/Game/1_UI/1_Textures/T_Icon_Betty.T_Icon_Betty")))