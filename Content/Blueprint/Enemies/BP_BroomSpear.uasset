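; Enemy broom spear projectile that strikes a target point and kills players caught in its landing radius.
; SetupSpear shows a landing warning widget, changes its state, then launches the spear after a short delay.
; A Timeline lerps it to the target, either dropping from high above with random roll or flying from its current position.
; On landing, a sphere trace calls player Death, a second Timeline animates rotation, and the actor expires after Lifetime.
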(event Custom|Landed
  (bind _returnvalue (Transformation|GetActorLocation))
  (Utilities|FlowControl|Sequence
    (:then_0
      (bind _outhits (Collision|MultiSphereTraceByChannel _returnvalue _returnvalue (Variables|Default|GetRadius) "TraceTypeQuery2" false 0 "None"))
      (for _array_element _outhits
        (bind _asbp_player (Utilities|Casting|CastToBP_Player (.HitActor (Collision|BreakHitResult _array_element))))
        (Default|Death _asbp_player))
      (Widget|RemovefromParent (Variables|Default|GetWidgetWarning))
      (Utilities|FlowControl|Delay (Variables|Default|GetLifetime))
      (Actor|DestroyActor))
    (:then_1
      (Variables|Default|SetInit_Rotate (Transformation|GetWorldRotation (Variables|Default|GetDefaultSceneRoot)))
      ;[1 1 1] Movement of Broom when is in the ground
      (bind _float (Timeline|Timeline_1 PlayFromStart)
        (:Update
          (Transformation|SetWorldRotation (Variables|Default|GetDefaultSceneRoot) (Math|Rotator|Lerp(Rotator) (Math|Rotator|MakeRotator (.roll (Variables|Default|GetInit_Rotate)) (.pitch (Variables|Default|GetInit_Rotate)) (.yaw (Variables|Default|GetInit_Rotate))) (Math|Rotator|MakeRotator (.roll (Variables|Default|GetInit_Rotate)) (+ (.roll (Variables|Default|GetInit_Rotate)) 1.0) (.yaw (Variables|Default|GetInit_Rotate))) _float) false false))))))

(event Custom|SetupSpear
  (params (EndPos :type Vector) (FromUp :type Boolean))
  (bind _output_get (Variables|Default|SetEndPos (Math|Vector|MakeVector (.x EndPos) (.y EndPos) (- (.z EndPos) 2e+01))))
  ;[1 0.5059 0.5059] Warning Widget
  (bind _returnvalue (UserInterface|CreateWidget "/Game/1_UI/3_Widgets/HUD/W_Warning.W_Warning_C" 0 self _output_get))
  (bind _output_get_2 (Variables|Default|SetWidgetWarning _returnvalue))
  (UserInterface|Viewport|AddtoViewport _output_get_2 0)
  (Utilities|FlowControl|Sequence
    (:then_0
      (Utilities|FlowControl|Delay 1.0)
      ;[1 0.5059 0.5059] Change Warning type
      (CallFunction|Launch FromUp))
    (:then_1
      (Utilities|FlowControl|Delay 0.35)
      (Default|ChangeWarning (Variables|Default|GetWidgetWarning) 1))))

(event Custom|Launch
  (params (FromUp :type Boolean))
  (if FromUp
    (Variables|Default|SetStartingPos (+ (Variables|Default|GetEndPos) "0.000000,0.000000,2000.000000"))
    (Transformation|SetActorRotation (Math|Rotator|MakeRotator (Math|Random|RandomFloatinRange -1.8e+02 1.8e+02) -9e+01 0.0))
    (bind _float (Timeline|Timeline PlayFromStart)
      (:Update
        (Transformation|SetActorLocation (Math|Vector|Lerp(Vector) (Variables|Default|GetStartingPos) (Variables|Default|GetEndPos) _float) false false))
      (:Finished
        (CallFunction|Landed)))
    (else
      (bind _output_get (Variables|Default|SetStartingPos (Transformation|GetWorldLocation (Variables|Default|GetDefaultSceneRoot))))
      (Transformation|SetWorldRotation (Variables|Default|GetDefaultSceneRoot) (Math|Rotator|FindLookatRotation _output_get (Variables|Default|GetEndPos)) false false)
      (Timeline|Timeline PlayFromStart))))

(event EventBeginPlay
  (Variables|Save|SetExist true))

(fn ConstructionScript)

(fn CheckIsCheckpointLoad
  (return false))