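; BP_Checkpoint is a checkpoint trigger that announces itself when the player enters its box.
; On overlap with BP_Player, it finds every actor implementing BPI_CheckpointInterface and sends UpdateCheckpointMessage with itself and a map name.
; GetLevelName derives that map name from its CurrentLevel variable by keeping the text after the last dot.
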(event OnComponentBeginOverlap(Box)
  (params (OverlappedComponent :type Primitive%20Component%20Object%20Reference) (OtherActor :type Actor%20Object%20Reference) (OtherComp :type Primitive%20Component%20Object%20Reference) (OtherBodyIndex :type Integer) (bFromSweep :type Boolean) (SweepResult :type Hit%20Result%20Structure%20%28by%20ref%29))
  (Utilities|Casting|CastToBP_Player OtherActor)
  (bind _outactors (Actor|GetAllActorswithInterface "/Game/Blueprint/CheckPoint/BPI_CheckpointInterface.BPI_CheckpointInterface_C"))
  (for _array_element _outactors
    (Class|BPICheckpointInterface|UpdateCheckpoint(Message) _array_element self (CallFunction|GetLevelName))))

(fn ConstructionScript)

(fn GetLevelName
  (bind _current_level (Variables|Default|GetCurrent%20Level))
  (bind _returnvalue (Utilities|ToString(SoftObjectReference) _current_level))
  (return (Utilities|String|StringToName (Utilities|String|GetSubstring _returnvalue (+ (Utilities|String|FindSubstring _returnvalue "." false true) 1) (Utilities|String|Len _returnvalue)))))