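; BP_RTC_CinematicPlayerJanitor is a cinematic trigger that plays a Level Sequence once, on player box overlap or shortly after BeginPlay if PlayOnStart disables the box.
; Unless IsRealTime, a CineCamera takes over from the player camera and glides to the Scene component's location via timeline before playback.
; PlayNewCinematic plays a supplied sequence without that move.
; With AutomaticEnd, a looping timer detects playback end, restores the player view and destroys the actor.
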(event OnComponentBeginOverlap(Box)
  (params (OverlappedComponent :type Primitive%20Component%20Object%20Reference) (OtherActor :type Actor%20Object%20Reference) (OtherComp :type Primitive%20Component%20Object%20Reference) (OtherBodyIndex :type Integer) (bFromSweep :type Boolean) (SweepResult :type Hit%20Result%20Structure%20%28by%20ref%29))
  (bind _returnvalue (Game|GetPlayerCharacter 0))
  (bind _cinecamera (Variables|Default|GetCineCamera))
  (bind _asbp_player (Utilities|Casting|CastToBP_Player _returnvalue))
  (bind _camera (Variables|/Game/Blueprint/Player/BP_Player.BP_Player_C|Getcamera _asbp_player))
  (bind _camera_2 (Variables|/Game/Blueprint/Camera/BP_Camera.BP_Camera_C|GetCamera _camera))
  ;[1 0 0 1 34] Trigger
  (Utilities|Casting|CastToBP_Player OtherActor)
  (Utilities|FlowControl|DoOnce false
    (:Completed
      (if (Variables|Default|GetisRealTime)
        (CallFunction|StartCinematic :!label _label)
        (else
          (Variables|Default|SetmoveCam true)
          (if (Variables|Default|GetmoveCam)
            (Transformation|SetWorldLocationAndRotation _cinecamera (Transformation|GetWorldLocation _camera_2) (Transformation|GetWorldRotation _camera_2) false false)
            (Game|Player|SetViewTargetwithBlend (Game|GetPlayerController 0) (Components|GetOwner _cinecamera) 0.0 "VTBlend_Linear" 0.0 false)
            (Utilities|FlowControl|DelayUntilNextTick)
            (bind _output_get (Variables|Default|SetfirstCineCamLoc (Transformation|GetWorldLocation (Variables|Default|GetCineCamera))))
            (bind _track (Timeline|Timeline PlayFromStart)
              (:Update
                (Transformation|SetWorldLocation (Variables|Default|GetCineCamera) (Math|Vector|Lerp(Vector) _output_get (Transformation|GetWorldLocation (Variables|Default|GetScene)) _track) false true))
              (:Finished
                (goto _label)))
            (else
              (goto _label))))))))

(event Custom|FinishCinematic
  ;[1 1 0 1 34] Cinematic
  (Game|Player|SetViewTargetwithBlend (Game|GetPlayerController 0) (Variables|/Game/Blueprint/Player/BP_Player.BP_Player_C|Getcamera (.AsBP%20Player (Utilities|Casting|CastToBP_Player (Game|GetPlayerCharacter 0)))) 0.0 "VTBlend_Linear" 0.0 false)
  (Actor|DestroyActor))

(event Custom|CheckFinishCinematic
  ;[1 1 0 1 34] Cinematic
  (if (not (Audio|Components|Audio|IsPlaying (stale Custom|StartCinematic _returnvalue)))
    (Game|Player|SetViewTargetwithBlend (Game|GetPlayerController 0) (Variables|/Game/Blueprint/Player/BP_Player.BP_Player_C|Getcamera (.AsBP%20Player (Utilities|Casting|CastToBP_Player (Game|GetPlayerCharacter 0)))) 0.0 "VTBlend_Linear" 0.0 false)
    (Actor|DestroyActor)))

(event Custom|StartCinematic
  ;[1 1 0 1 34] Cinematic
  (bind _returnvalue (Sequencer|Player|CreateLevelSequencePlayer (Variables|Default|GetlevelSequence)))
  (Sequencer|Player|Play _returnvalue :!class /Script/MovieScene.MovieSceneSequencePlayer)
  (if (Variables|Default|GetautomaticEnd)
    (Utilities|Time|SetTimerbyEvent (delegate Custom|CheckFinishCinematic) 0.1 true)))

(event Custom|PlayNewCinematic
  (params (levelSequence :type Level%20Sequence%20Object%20Reference))
  (bind _returnvalue (Game|GetPlayerCharacter 0))
  (bind _cinecamera (Variables|Default|GetCineCamera))
  (bind _asbp_player (Utilities|Casting|CastToBP_Player _returnvalue))
  (bind _camera (Variables|/Game/Blueprint/Player/BP_Player.BP_Player_C|Getcamera _asbp_player))
  (bind _camera_2 (Variables|/Game/Blueprint/Camera/BP_Camera.BP_Camera_C|GetCamera _camera))
  ;[1 0 0 1 34] Trigger
  (Variables|Default|SetlevelSequence levelSequence)
  (Variables|Default|SetmoveCam false)
  (if (Variables|Default|GetmoveCam)
    (Transformation|SetWorldLocationAndRotation _cinecamera (Transformation|GetWorldLocation _camera_2) (Transformation|GetWorldRotation _camera_2) false false)
    (Game|Player|SetViewTargetwithBlend (Game|GetPlayerController 0) (Components|GetOwner _cinecamera) 0.0 "VTBlend_Linear" 0.0 false)
    (Utilities|FlowControl|DelayUntilNextTick)
    (bind _output_get (Variables|Default|SetfirstCineCamLoc (Transformation|GetWorldLocation (Variables|Default|GetCineCamera))))
    (bind _track (Timeline|Timeline PlayFromStart)
      (:Update
        (Transformation|SetWorldLocation (Variables|Default|GetCineCamera) (Math|Vector|Lerp(Vector) _output_get (Transformation|GetWorldLocation (Variables|Default|GetScene)) _track) false true))
      (:Finished
        (CallFunction|StartCinematic :!label _label)))
    (else
      (goto _label))))

(event EventBeginPlay
  (bind _returnvalue (Game|GetPlayerCharacter 0))
  (bind _cinecamera (Variables|Default|GetCineCamera))
  (bind _asbp_player (Utilities|Casting|CastToBP_Player _returnvalue))
  (bind _camera (Variables|/Game/Blueprint/Player/BP_Player.BP_Player_C|Getcamera _asbp_player))
  (bind _camera_2 (Variables|/Game/Blueprint/Camera/BP_Camera.BP_Camera_C|GetCamera _camera))
  ;[1 0 0 1 34] Trigger
  (if (Variables|Default|GetplayOnStart)
    (Utilities|FlowControl|Delay 0.2)
    (Utilities|FlowControl|DoOnce false
      (:Completed
        (if (Variables|Default|GetisRealTime)
          (CallFunction|StartCinematic :!label _label)
          (else
            (Variables|Default|SetmoveCam true)
            (if (Variables|Default|GetmoveCam)
              (Transformation|SetWorldLocationAndRotation _cinecamera (Transformation|GetWorldLocation _camera_2) (Transformation|GetWorldRotation _camera_2) false false)
              (Game|Player|SetViewTargetwithBlend (Game|GetPlayerController 0) (Components|GetOwner _cinecamera) 0.0 "VTBlend_Linear" 0.0 false)
              (Utilities|FlowControl|DelayUntilNextTick)
              (bind _output_get (Variables|Default|SetfirstCineCamLoc (Transformation|GetWorldLocation (Variables|Default|GetCineCamera))))
              (bind _track (Timeline|Timeline PlayFromStart)
                (:Update
                  (Transformation|SetWorldLocation (Variables|Default|GetCineCamera) (Math|Vector|Lerp(Vector) _output_get (Transformation|GetWorldLocation (Variables|Default|GetScene)) _track) false true))
                (:Finished
                  (goto _label)))
              (else
                (goto _label)))))))))

(fn ConstructionScript
  (bind _box (Variables|Default|GetBox))
  (Collision|SetCollisionEnabled _box (select (Variables|Default|GetplayOnStart) "NoCollision" "QueryOnly"))
  (Rendering|SetVisibility _box (not (Variables|Default|GetplayOnStart)) false))