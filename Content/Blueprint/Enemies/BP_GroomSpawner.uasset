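; BP_GroomSpawner is a trigger volume that spawns a BP_Groom enemy at its SpawnPoint when the player first overlaps the box.
; It passes FirstBehaviour and a start delay equal to the optional montage's length, or one second without a montage.
; With a valid montage, it plays it on the groom's mesh and destroys itself immediately, without waiting for completion; otherwise DoOnce prevents repeat spawns.
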(event OnComponentBeginOverlap(Box)
  (params (OverlappedComponent :type Primitive%20Component%20Object%20Reference) (OtherActor :type Actor%20Object%20Reference) (OtherComp :type Primitive%20Component%20Object%20Reference) (OtherBodyIndex :type Integer) (bFromSweep :type Boolean) (SweepResult :type Hit%20Result%20Structure%20%28by%20ref%29))
  (Utilities|Casting|CastToBP_Player OtherActor)
  (Utilities|FlowControl|DoOnce false
    (:Completed
      (bind _returnvalue (Game|SpawnActorfromClass "/Game/Blueprint/Enemies/BP_Groom.BP_Groom_C" (Transformation|GetWorldTransform (Variables|Default|GetSpawnPoint)) "Undefined" "MultiplyWithRoot" 0 (Variables|Default|GetfirstBehaviour) (select (Utilities|IsValid (Variables|Default|GetmontageToPlay)) (Variables|/Script/Engine.AnimSequenceBase|GetSequenceLength (Variables|Default|GetmontageToPlay)) 1.0) 0))
      (bind _montagetoplay (Variables|Default|GetmontageToPlay)
        (:then
          (Animation|Montage|PlayMontage (Variables|/Script/Engine.Character|GetMesh _returnvalue) _montagetoplay
            (:then
              (Actor|DestroyActor))))
        (:else)))))

(fn ConstructionScript)