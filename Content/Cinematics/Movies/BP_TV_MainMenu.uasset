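; BP_TV_MainMenu is a main-menu TV that plays a looping screen-recording video after a material transition.
; One second after BeginPlay, the ChangeProgress timeline drives the Progress scalar on the Plane's materials.
; A short Delay chained to the timeline's Update, rather than Finished, swaps the Plane to MI_TV_Inst and opens the video on TVMediaPlayer, so both can repeat while the timeline runs.
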(event EventBeginPlay
  (Utilities|FlowControl|Delay 1.0)
  (bind _progress (Timeline|Change%20Progress PlayFromStart)
    (:Update
      (Rendering|Material|SetScalarParameterValueonMaterials (Variables|Default|GetPlane) "Progress" _progress)
      (Utilities|FlowControl|Delay 0.3)
      (Rendering|Material|SetMaterial (Variables|Default|GetPlane) 0 "/Game/Cinematics/Movies/MI_TV_Inst.MI_TV_Inst")
      (Media|MediaPlayer|OpenSource (Variables|Default|GetTV%20Media%20Player) "/Game/Cinematics/Movies/Enregistrement_de_l_écran_2025-03-26_161304.Enregistrement_de_l_écran_2025-03-26_161304")
      (Components|Timeline|SetLooping (Variables|Default|GetTV%20Media%20Player) true))))

(fn ConstructionScript)