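; Minion character that trails the player at an Index-based offset, re-pathing through a behaviour loop and sprinting when the player sprints or gets too far away.
; When Climb is triggered, it faces the player and, while airborne, either follows a Drawer's spline or checks for a climbable target.
; Timelines drive climbs, edge jumps and drawer jumps, with drawer changes during jumps buffered until landing.
; The Interact behaviour only prints a debug string.
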(event Custom|Sprint
  (bind _charactermovement (Variables|Character|GetCharacterMovement))
  ;[1 1 1] Sprint
  (if (CallFunction|CanSprint)
    (Variables|/Script/Engine.CharacterMovementComponent|SetMaxWalkSpeed _charactermovement 7.5e+02)
    (else
      (Variables|/Script/Engine.CharacterMovementComponent|SetMaxWalkSpeed _charactermovement 5e+02))))

(event Custom|Climb
  ;[0.1569 0.07843 0 1 34] Climb
  (Variables|Default|SetcanCheckClimb true))

(event Custom|PickDecision
  (params (currentBehaviour :type Enum_MinionsBehaviour%20Enum :default "NewEnumerator0"))
  ;[0 0.2 0 1 34] Pick decision
  (bind _output_get (Variables|Default|SetcurrentBehaviour currentBehaviour))
  (switch Utilities|FlowControl|Switch|SwitchonEnum_MinionsBehaviour _output_get
    (:NewEnumerator0
      (CallFunction|FollowPlayer))
    (:NewEnumerator1
      (CallFunction|Interact))))

(event Custom|CheckClimb
  ;[0.1569 0.07843 0 1 34] Climb
  (if (AI|Components|NavMovement|IsMovingonGround (Variables|Character|GetCharacterMovement))
    (Variables|Default|SetcanCheckClimb false)
    (else
      (Utilities|IsValid (Variables|Default|GetDrawer)
        (:Is%20Valid
          (CallFunction|JumpDrawer))
        (:Is%20Not%20Valid
          (bind (_canclimb _target) (CallFunction|Climb (Transformation|GetActorLocation) (Transformation|GetActorForwardVector) (Transformation|GetActorUpVector) "None"))
          (if _canclimb
            (Utilities|FlowControl|DoOnce false :!label _label
              (:Completed
                (Variables|Default|SetcanCheckClimb false)
                (Pawn|Components|CharacterMovement|SetMovementMode (Variables|Character|GetCharacterMovement) "MOVE_Flying" 0)
                (Variables|Default|SetisClimbing true)
                (Variables|Default|SetfirstClimbLoc (Transformation|GetActorLocation))
                (Variables|Default|SetendClimbLoc _target)
                (bind _track (Timeline|Timeline_Climb PlayFromStart)
                  (:Update
                    (Transformation|SetActorLocation (Math|Vector|Lerp(Vector) (Variables|Default|GetfirstClimbLoc) (Variables|Default|GetendClimbLoc) _track) false true))
                  (:Finished
                    (Variables|Default|SetisClimbing false)
                    (Pawn|Components|CharacterMovement|SetMovementMode (Variables|Character|GetCharacterMovement) "MOVE_Walking" 0)
                    (goto _label Reset)))))))))))

(event Custom|Interact
  ;[0 1 1 1 34] Interact
  (Development|PrintString "Interact Minion"))

(event Custom|EdgeJump
  (params (targetLoc :type Vector))
  ;[1 0.6667 0 1 34] Edge jump (follow player)
  (Utilities|FlowControl|DoOnce false :!label _label
    (:Completed
      (Character|Jump)
      (Utilities|FlowControl|Delay 0.2)
      (Variables|Default|SetfirstJumpLoc (Transformation|GetActorLocation))
      (Variables|Default|SetIsJummping true)
      (bind _track (Timeline|Timeline_EdgeJump PlayFromStart)
        (:Update
          (Transformation|SetActorLocationAndRotation (Math|Vector|Lerp(Vector) (Variables|Default|GetfirstJumpLoc) targetLoc _track) (Math|Rotator|MakeRotator (.roll (Math|Rotator|FindLookatRotation (Variables|Default|GetfirstJumpLoc) targetLoc)) (.pitch (Math|Rotator|FindLookatRotation (Variables|Default|GetfirstJumpLoc) targetLoc)) (.yaw (Math|Rotator|FindLookatRotation (Variables|Default|GetfirstJumpLoc) targetLoc)))))
        (:Finished
          (Variables|Default|SetIsJummping false)
          (CallFunction|FollowPlayer)
          (Transformation|SetActorRotation (Math|Rotator|MakeRotator 0.0 0.0 (.yaw (Math|Rotator|FindLookatRotation (Variables|Default|GetfirstJumpLoc) targetLoc))))
          (Utilities|FlowControl|Delay 0.2)
          (goto _label Reset))))))

(event Custom|FollowPlayer
  (bind _playerref (Variables|Default|GetPlayerRef))
  ;[0 1 0 1 34] Follow player
  (if (not (Variables|Default|GetIsJummping))
    (switch Utilities|FlowControl|Switch|SwitchonEnum_MinionsBehaviour (Variables|Default|GetcurrentBehaviour)
      (:NewEnumerator0
        (AI|Navigation|SimpleMovetoLocation (Pawn|GetController) (- (Transformation|GetActorLocation _playerref) (* (Transformation|GetActorForwardVector _playerref) (* (+ (Variables|Default|Getindex) 1) 1.5e+02))))
        (Utilities|FlowControl|Delay 0.1)
        (switch Utilities|FlowControl|Switch|SwitchonEnum_MinionsBehaviour (Variables|Default|GetcurrentBehaviour)
          (:NewEnumerator0
            (CallFunction|PickDecision "NewEnumerator0")))))))

(event Custom|JumpDrawer
  (Utilities|FlowControl|DoOnce false :!label _label
    (:Completed
      (Variables|Default|SetIsJummping true)
      (bind _spline (Default|GetSpline (Variables|Default|GetDrawer) (Variables|Default|GetDrawer%20Side)))
      (Variables|Default|SetDrawer%20Side (Variables|Default|GetDrawer%20Side))
      (bind _time (Timeline|Timeline PlayFromStart)
        (:Update
          (Transformation|SetActorLocation (CallFunction|GetRelativeDrawerAnim _time _spline) false false))
        (:Finished
          (Variables|Default|SetIsJummping false)
          (CallFunction|FollowPlayer)
          (Variables|Default|SetDrawer%20Side (Variables|Default|GetDrawerSideTemp))
          (Variables|Default|SetDrawer (Variables|Default|GetDrawerTemp))
          (goto _label Reset))))))

(event EventSetupDrawer
  (params (Drawer :type BP%20Drawer%20Object%20Reference) (DrawerSide :type E_DrawerSIde%20Enum :default "NewEnumerator3"))
  (if (Variables|Default|GetIsJummping)
    (Variables|Default|SetDrawerTemp Drawer)
    (Variables|Default|SetDrawerSideTemp DrawerSide)
    (else
      (Variables|Default|SetDrawer Drawer)
      (Variables|Default|SetDrawer%20Side DrawerSide))))

(event EventClimbtoPoint
  (params (cable :type BP%20Rope%20Object%20Reference))
  ;[0.1569 0.07843 0 1 34] Climb
)

(event EventBeginPlay
  ;[0 0 0 1 34] Start
  (bind _asbp_player (Utilities|Casting|CastToBP_Player (Game|GetPlayerCharacter 0)))
  (Variables|Default|SetPlayerRef _asbp_player)
  (CallFunction|PickDecision "NewEnumerator0")
  (AI|SetFocus (AI|GetAIController self) (Variables|Default|GetPlayerRef)))

(event EventTick
  (params (DeltaSeconds :type Float%20%28single-precision%29))
  (bind _returnvalue (Transformation|GetActorRotation))
  ;[0 0 0 1 34] Update
  (CallFunction|Sprint)
  (if (Variables|Default|GetcanCheckClimb)
    (Transformation|SetActorRotation (Math|Rotator|MakeRotator (.roll _returnvalue) (.pitch _returnvalue) (.yaw (Math|Rotator|FindLookatRotation (Transformation|GetActorLocation) (Transformation|GetActorLocation (Variables|Default|GetPlayerRef))))) true)
    (CallFunction|CheckClimb)))

(fn ConstructionScript)

(fn GetRelativeDrawerAnim
  (params (Time :type Float%20%28single-precision%29) (Spine :type Spline%20Component%20Object%20Reference))
  (bind _returnvalue (Spline|GetLocationatTime Spine Time "World" false))
  (bind _returnvalue_2 (Transformation|GetActorLocation))
  (bind _drawer_side (Variables|Default|GetDrawer%20Side))
  (return (Math|Vector|MakeVector (Utilities|Select :Index _drawer_side :NewEnumerator3 0.0 :NewEnumerator0 (.x _returnvalue) :NewEnumerator1 (.x _returnvalue_2) :NewEnumerator2 (.x _returnvalue_2)) (Utilities|Select :Index _drawer_side :NewEnumerator3 0.0 :NewEnumerator0 (.y _returnvalue_2) :NewEnumerator1 (.y _returnvalue) :NewEnumerator2 (.y _returnvalue)) (.z _returnvalue))))

(fn CanSprint
  (return (or (== (Variables|/Script/Engine.CharacterMovementComponent|GetMaxWalkSpeed (Variables|/Script/Engine.Character|GetCharacterMovement (Variables|Default|GetPlayerRef))) 7.5e+02) (> (Transformation|GetDistanceTo (Variables|Default|GetPlayerRef) self) 5e+02))))