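; BP_SlipperyFloor is a level element that makes the player slip while standing inside its Box trigger.
; On begin overlap it registers itself in the BP_Player's SlipperyFloors array and turns slippering on if it is not already active.
; On end overlap it removes itself and turns slippering off only when the array is empty, so overlapping or adjacent floors keep the effect continuous.
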(event OnComponentBeginOverlap(Box)
  (params (OverlappedComponent :type Primitive%20Component%20Object%20Reference) (OtherActor :type Actor%20Object%20Reference) (OtherComp :type Primitive%20Component%20Object%20Reference) (OtherBodyIndex :type Integer) (bFromSweep :type Boolean) (SweepResult :type Hit%20Result%20Structure%20%28by%20ref%29))
  (bind _self self)
  ;[1 0 0 1 34] Trigger
  (bind _asbp_player (Utilities|Casting|CastToBP_Player OtherActor))
  (if (not (Utilities|Array|ContainsItem (Variables|/Game/Blueprint/Player/BP_Player.BP_Player_C|GetslipperyFloors _asbp_player) _self))
    (Utilities|Array|AddUnique (Variables|/Game/Blueprint/Player/BP_Player.BP_Player_C|GetslipperyFloors _asbp_player) _self)
    (if (not (Variables|/Game/Blueprint/Player/BP_Player.BP_Player_C|GetisSlippering _asbp_player))
      (Default|SetSlippering _asbp_player true))))

(event OnComponentEndOverlap(Box)
  (params (OverlappedComponent :type Primitive%20Component%20Object%20Reference) (OtherActor :type Actor%20Object%20Reference) (OtherComp :type Primitive%20Component%20Object%20Reference) (OtherBodyIndex :type Integer))
  (bind _self self)
  ;[1 0 0 1 34] Trigger
  (bind _asbp_player (Utilities|Casting|CastToBP_Player OtherActor))
  (if (Utilities|Array|ContainsItem (Variables|/Game/Blueprint/Player/BP_Player.BP_Player_C|GetslipperyFloors _asbp_player) _self)
    (Utilities|Array|RemoveItem (Variables|/Game/Blueprint/Player/BP_Player.BP_Player_C|GetslipperyFloors _asbp_player) _self)
    (if (<= (Utilities|Array|Length (Variables|/Game/Blueprint/Player/BP_Player.BP_Player_C|GetslipperyFloors _asbp_player)) 0)
      (Default|SetSlippering _asbp_player false))))

(fn ConstructionScript)