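; Lobby cinematic manager that steps through indexed level sequences and dialogues via its cinematic and dialogue players.
; It registers with GI_Instance either at BeginPlay, hiding the player mesh unless a checkpoint is loading, or through a one-shot trigger box, as SetOnStart selects.
; Events handle camera shake, Karl's HUD icon, the loading screen, and end-of-cinematic visibility.
; A DoOnce with delayed reset debounces sequence starts.
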(event OnComponentBeginOverlap(Box)
  (params (OverlappedComponent :type Primitive%20Component%20Object%20Reference) (OtherActor :type Actor%20Object%20Reference) (OtherComp :type Primitive%20Component%20Object%20Reference) (OtherBodyIndex :type Integer) (bFromSweep :type Boolean) (SweepResult :type Hit%20Result%20Structure%20%28by%20ref%29))
  ;[1 0 0 1 34] Box
  (Utilities|Casting|CastToBP_Player OtherActor)
  (bind _asgi_instance (Utilities|Casting|CastToGI_Instance (Game|GetGameInstance)))
  (Variables|/Game/Blueprint/GI_Instance.GI_Instance_C|SetcinematicManager _asgi_instance self)
  (Components|DestroyComponent (Variables|Default|GetBox)))

(event Custom|CameraShake
  ;[0 0 1 1 34] Camera event
  (CameraShakes|StartCameraShake (Game|GetPlayerCameraManager 0) "/Game/Blueprint/Camera/CS_GroomFall.CS_GroomFall_C" 1.0 "CameraLocal" "0, 0, 0"))

(event Custom|FinishCinematic
  ;[1 1 0 1 34] Cinematic event
  (bind _asbp_player (Utilities|Casting|CastToBP_Player (Game|GetPlayerCharacter 0)))
  (Rendering|SetVisibility (Variables|/Script/Engine.Character|GetMesh _asbp_player) true false)
  (Default|FinishCinematic (Variables|Default|GetcinematicPlayer))
  (Default|Show/HideMinions _asbp_player false)
  (Utilities|FlowControl|Delay 0.5)
  (Rendering|SetVisibility (Variables|/Script/Engine.SkeletalMeshActor|GetSkeletalMeshComponent (Variables|Default|GetKarl)) false false))

(event Custom|NewCinematic
  ;[1 1 0 1 34] Cinematic event
  (Utilities|FlowControl|DoOnce false :!label _label
    (:Completed
      (Default|PlayNewCinematic (Variables|Default|GetcinematicPlayer) (Utilities|Array|Get(acopy) (Variables|Default|GetLevel%20Sequence) (Variables|Default|GetindexLevelSequence)))
      (Math|Integer|IncrementInt (Variables|Default|GetindexLevelSequence)
        (:%20%20
          (Utilities|FlowControl|Delay 0.5)
          (goto _label Reset))))))

(event Custom|SetNewDialogue
  ;[0 1 0 1 34] Dialogue event
  ;;[1 0 0] BUG ICI DESFOIS_ N'a pas la référence de dialogue player
  (Default|SetNewDialogue (Variables|Default|GetdialoguePlayer) (Utilities|Array|Get(acopy) (Variables|Default|Getdialogues) (Variables|Default|GetindexDialogue)))
  (Math|Integer|IncrementInt (Variables|Default|GetindexDialogue)))

(event Custom|SetNewFriendsKarl
  (bind _asbp_player (Utilities|Casting|CastToBP_Player (Game|GetPlayerCharacter 0)))
  (Default|SetNewElement (Variables|/Game/Blueprint/Player/BP_Player.BP_Player_C|GetHUD _asbp_player) (Utilities|Struct|MakeStruct_Collectible "NewEnumerator0" "NewEnumerator0" "/Game/1_UI/1_Textures/T_Icon_Karl.T_Icon_Karl" 0 0)))

(event Custom|Transition
  (bind _returnvalue (UserInterface|CreateWidget "/Game/1_UI/3_Widgets/Loading/W_LoadingScreen.W_LoadingScreen_C" 0 1))
  (UserInterface|Viewport|AddtoViewport _returnvalue 0))

(event EventBeginPlay
  ;[0 0 0 1 34] Start
  (bind _ischeckpointload (Class|BPICheckpointInterface|CheckIsCheckpointLoad(Message) (Game|GetGameMode)))
  (if (not _ischeckpointload)
    (if (Variables|Default|GetsetOnStart)
      (bind _asbp_player (Utilities|Casting|CastToBP_Player (Game|GetPlayerCharacter 0)))
      (Rendering|SetVisibility (Variables|/Script/Engine.Character|GetMesh _asbp_player) false false)
      (bind _asgi_instance (Utilities|Casting|CastToGI_Instance (Game|GetGameInstance)))
      (Variables|/Game/Blueprint/GI_Instance.GI_Instance_C|SetcinematicManager _asgi_instance self))))

(fn ConstructionScript
  (bind _box (Variables|Default|GetBox))
  (bind _setonstart (Variables|Default|GetsetOnStart))
  (Rendering|SetVisibility _box (not _setonstart) false)
  (Collision|SetCollisionEnabled _box (select _setonstart "NoCollision" "QueryOnly")))