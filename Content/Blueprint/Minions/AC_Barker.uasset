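; AC_Barker is a component that lets its owning character, likely a minion, bark multi-line dialogue, either a given bark or a random pick from a list or its defaults.
; Bark currently only debug-prints the joined lines for their summed duration.
; An unconnected draft shows a WBP_Bark bubble above the owner, with timers intended to step through lines via ContinueBark and close it via EndBark.
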(event EventBeginPlay
  (Variables|ObjectRefs|SetOwner (Components|GetOwner)))

(event EventTick
  (params (DeltaSeconds :type Float%20%28single-precision%29)))

(fn Bark
  (params (InputBark :type F%20Bark%20Structure))
  (bind (_lines _durations) (Utilities|Struct|BreakF_Bark InputBark))
  ;[1 0 0.01785] DEBUG - this will normally cycle through each bark, writing it to a generated UI above the barker's head. There will be no need for variables such as TotalBark, TotalDuration or CharacterName in later versions.
  (for (_array_element _array_index) _lines
    (LocalVariables|SetTotalBark (Utilities|String|Append (LocalVariables|GetTotalBark) " " (Utilities|String|ToString(Text) _array_element)))
    (LocalVariables|SetTotalDuration (+ (LocalVariables|GetTotalDuration) (Utilities|Array|Get(acopy) _durations _array_index))))
  (Development|PrintString (Utilities|String|Append (Variables|Parameters|GetCharacterName) " barked: \"" (LocalVariables|GetTotalBark)) true true "(R=0.493130,G=0.000000,B=1.000000,A=1.000000)" (LocalVariables|GetTotalDuration) (Utilities|String|StringToName (Utilities|String|Append (Variables|Parameters|GetCharacterName) "BarkDEBUG"))))

(fn RandomBark
  (params (BarkList :type Array%20of%20F%20Bark%20Structures))
  (Barking|Bark (Utilities|Array|Get(acopy) BarkList (Math|Random|RandomIntegerinRange 0 (- (Utilities|Array|Length BarkList) 1)))))

(fn RandomDefaultBark
  (Barking|RandomBark (Variables|Barks|GetDefaultBarks)))

(fn EndBark
  (Default|Disappear (Variables|ObjectRefs|GetBarkWidget))
  (Variables|ObjectRefs|SetBarkWidget 0)
  (Variables|Private|SetCurrentBark (Utilities|Struct|MakeF_Bark 0 "(3.000000)")))

(fn ContinueBark
  (bind _currentbark (Variables|Private|GetCurrentBark))
  (bind (_lines _durations) (Utilities|Struct|BreakF_Bark _currentbark))
  (bind _result (Math|Integer|IncrementInt (Variables|Private|GetCurrentBarkIndex))
    (:%20%20
      (if (>= _result (Utilities|Array|Length _lines))
        (CallFunction|EndBark)
        (else
          (Default|PopulateBark (Variables|ObjectRefs|GetBarkWidget) (Utilities|Array|Get(acopy) _lines _result))
          (bind _returnvalue (Utilities|Time|SetTimerbyEvent (EventDispatchers|CreateEvent :!event ContinueBark) (Utilities|Array|Get(acopy) _durations _result)))
          (Variables|Private|SetBarkTimer _returnvalue))))))