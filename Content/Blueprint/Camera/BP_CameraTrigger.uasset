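; BP_CameraTrigger is a box volume that registers itself in the player's camera trigger list while BP_Player overlaps it.
; An Override trigger inserts itself at the front of the list, others are appended uniquely, and leaving the box removes the trigger.
; On BeginPlay, the box's collision is switched off and restored as query-only after a short delay.
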(event OnComponentEndOverlap(Box)
  (params (OverlappedComponent :type Primitive%20Component%20Object%20Reference) (OtherActor :type Actor%20Object%20Reference) (OtherComp :type Primitive%20Component%20Object%20Reference) (OtherBodyIndex :type Integer))
  (bind _asbp_player (Utilities|Casting|CastToBP_Player OtherActor))
  (Utilities|Array|RemoveItem (Variables|/Game/Blueprint/Camera/BP_Camera.BP_Camera_C|GetCameraTriggers (Variables|/Game/Blueprint/Player/BP_Player.BP_Player_C|Getcamera _asbp_player)) self))

(event OnComponentBeginOverlap(Box)
  (params (OverlappedComponent :type Primitive%20Component%20Object%20Reference) (OtherActor :type Actor%20Object%20Reference) (OtherComp :type Primitive%20Component%20Object%20Reference) (OtherBodyIndex :type Integer) (bFromSweep :type Boolean) (SweepResult :type Hit%20Result%20Structure%20%28by%20ref%29))
  (bind _self self)
  (bind _asbp_player (Utilities|Casting|CastToBP_Player OtherActor))
  (if (Variables|Params|GetOverride)
    (Utilities|Array|Insert (Variables|/Game/Blueprint/Camera/BP_Camera.BP_Camera_C|GetCameraTriggers (Variables|/Game/Blueprint/Player/BP_Player.BP_Player_C|Getcamera _asbp_player)) _self)
    (else
      (Utilities|Array|AddUnique (Variables|/Game/Blueprint/Camera/BP_Camera.BP_Camera_C|GetCameraTriggers (Variables|/Game/Blueprint/Player/BP_Player.BP_Player_C|Getcamera _asbp_player)) _self))))

(event EventBeginPlay
  (Collision|SetCollisionEnabled (Variables|Default|GetBox) "NoCollision")
  (Utilities|FlowControl|Delay 0.1)
  (Collision|SetCollisionEnabled (Variables|Default|GetBox) "QueryOnly"))

(fn ConstructionScript)