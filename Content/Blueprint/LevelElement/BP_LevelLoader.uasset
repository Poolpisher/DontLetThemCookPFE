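; Level transition actor that swaps streamed levels when the player enters its box and places the player on arrival.
; On BeginPlay it saves its CurrentLevel name in the game instance and, if enabled and CanTP, teleports the player to PlayerStart and calls SetMinions.
; On overlap with CanTP, it force-finishes any dialogue, then streams in LevelToLoad and unloads CurrentLevel behind a delayed loading screen.
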(event OnComponentBeginOverlap(Box)
  (params (OverlappedComponent :type Primitive%20Component%20Object%20Reference) (OtherActor :type Actor%20Object%20Reference) (OtherComp :type Primitive%20Component%20Object%20Reference) (OtherBodyIndex :type Integer) (bFromSweep :type Boolean) (SweepResult :type Hit%20Result%20Structure%20%28by%20ref%29))
  ;[1 0.3333 0 1 34] Load level
  (bind _asbp_player (Utilities|Casting|CastToBP_Player OtherActor))
  (Variables|Default|GetlevelToLoad
    (:then
      (if (Variables|Default|GetcanTP)
        (bind _currentdialogue (Variables|/Game/Blueprint/Player/BP_Player.BP_Player_C|GetcurrentDialogue _asbp_player)
          (:then
            (Default|ForceFinishDialogue _currentdialogue))
          (:else
            _))
        (bind _returnvalue (UserInterface|CreateWidget "/Game/1_UI/3_Widgets/Loading/W_LoadingScreen.W_LoadingScreen_C" 0 (Variables|Default|GetloadAnim)))
        (bind _output_get (Variables|Default|SetloadingScreen _returnvalue))
        (UserInterface|Viewport|AddtoViewport _output_get 0)
        (Utilities|FlowControl|Delay 1.0)
        (Class|GameplayStatics|LoadStreamLevelbySoftObjectPtr (Variables|Default|GetlevelToLoad) true false)
        (Utilities|FlowControl|Delay 0.5)
        (Default|FinishLoad (Variables|Default|GetloadingScreen))
        (Class|GameplayStatics|UnloadStreamLevelbySoftObjectPtr (Variables|Default|GetcurrentLevel) false)))
    (:else)))

(event EventBeginPlay
  (bind _returnvalue (Game|GetPlayerCharacter 0))
  ;[0 0 0 1 34] Start
  (Variables|/Game/Blueprint/GI_Instance.GI_Instance_C|SetcurrentLevel (.AsGI%20Instance (Utilities|Casting|CastToGI_Instance (Game|GetGameInstance))) (Utilities|String|StringToName (Utilities|String|GetSubstring (Utilities|ToString(SoftObjectReference) (Variables|Default|GetcurrentLevel)) (+ (Utilities|String|FindSubstring (Utilities|ToString(SoftObjectReference) (Variables|Default|GetcurrentLevel)) "." false true) 1) (Utilities|String|Len (Utilities|ToString(SoftObjectReference) (Variables|Default|GetcurrentLevel)))))) ; Save current level in instance
  (if (Variables|Default|GetisEnable)
    (if (Variables|Default|GetcanTP)
      (Utilities|IsValid _returnvalue
        (:Is%20Valid
          (Transformation|SetActorLocation _returnvalue (Transformation|GetWorldLocation (Variables|Default|GetPlayerStart)) false true)
          (bind _asbp_player (Utilities|Casting|CastToBP_Player (Game|GetPlayerCharacter 0)))
          (Default|SetMinions _asbp_player))))))

(fn ConstructionScript)