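; Movement function library whose Climb function tests whether a climb is possible from a given location and returns a target point.
; A forward visibility line trace must hit an actor tagged "Climb".
; A second, raised trace along the combined forward and up direction must then be clear, and its end point becomes the target.
; Both traces take a debug draw option from the caller.
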(fn Climb
  (params (location :type Vector) (forward :type Vector) (up :type Vector) (debug :type EDrawDebugTrace%20Enum :default "None"))
  (bind _returnvalue (+ location "0.000000,0.000000,80.000000"))
  (bind _outhit (Collision|LineTraceByChannel 0 location (+ location (* forward 1.5e+02)) "TraceTypeQuery1" false 0 debug true "(R=1.000000,G=0.000000,B=0.000000,A=1.000000)" "(R=0.000000,G=1.000000,B=0.000000,A=1.000000)" 2.0))
  (if (.bBlockingHit (Collision|BreakHitResult _outhit))
    (if (Actor|ActorHasTag (.HitActor (Collision|BreakHitResult _outhit)) "Climb")
      (bind _outhit_2 (Collision|LineTraceByChannel 0 _returnvalue (+ _returnvalue (* (+ forward up) 1.8e+02)) "TraceTypeQuery1" false 0 debug true "(R=0.004252,G=0.000000,B=1.000000,A=1.000000)" "(R=0.000000,G=0.700514,B=1.000000,A=1.000000)" 2.0))
      (return (not (.bBlockingHit (Collision|BreakHitResult _outhit_2))) (.TraceEnd (Collision|BreakHitResult _outhit_2)))
      (else
        (return false "0, 0, 0")))
    (else
      (return false "0, 0, 0"))))