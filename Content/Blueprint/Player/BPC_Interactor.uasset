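; Player interaction component that tracks and highlights the nearest interactable around the player character.
; Each tick while CanInteract is set, a sphere overlap gathers BPI_Interact actors, skipping BPP_InteractableParent ones flagged non-interactable, and picks the closest.
; A new pick receives SelectMessage; DeselectMessage fires only when none is found or interaction is disabled, not when switching between targets.
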(event EventTick
  (params (DeltaSeconds :type Float%20%28single-precision%29))
  (if (Variables|Parameters|GetCanInteract?)
    (CallFunction|HandleCurrentlySelectedInteractible)
    (else
      (bind _currentlyselectedinteractible (Variables|Interactible|GetCurrentlySelectedInteractible)
        (:then
          (Class|BPIInteract|Deselect(Message) _currentlyselectedinteractible)
          (Variables|Interactible|SetCurrentlySelectedInteractible 0))
        (:else)))))

(fn InitializeComponent
  (bind _asbp_player (Utilities|Casting|CastToBP_Player (Game|GetPlayerCharacter 0)))
  (Variables|ObjectRefs|SetPlayer _asbp_player))

(fn HandleCurrentlySelectedInteractible
  (bind _player (Variables|ObjectRefs|GetPlayer)
    (:then
      (bind _outactors (Collision|SphereOverlapActors (Transformation|GetActorLocation _player) (Variables|Parameters|GetDetectionRange) (Utilities|Array|MakeArray "ObjectTypeQuery2" "ObjectTypeQuery3") 0))
      ;[0 0 0 1 34] Select interactible
      (for _array_element _outactors
        (if (Utilities|DoesObjectImplementInterface _array_element "/Game/Blueprint/Interactables/BPI_Interact.BPI_Interact_C")
          (bind _asbpp_interactable_parent (Utilities|Casting|CastToBPP_InteractableParent _array_element)
            (:then
              (if (Variables|/Game/Blueprint/Interactables/BPP_InteractableParent.BPP_InteractableParent_C|GetCanBeInteractedWith? _asbpp_interactable_parent)
                (Utilities|Array|AddUnique (LocalVariables|GetFoundInteractibles) _array_element :!label _label)))
            (:CastFailed
              (goto _label)))))
      (for _array_element_2 (LocalVariables|GetFoundInteractibles)
        (if (< (Math|Vector|Distance(Vector) (Transformation|GetActorLocation _array_element_2) (Transformation|GetActorLocation (Variables|ObjectRefs|GetPlayer))) (LocalVariables|GetClosestDistance))
          (LocalVariables|SetClosestDistance (Math|Vector|Distance(Vector) (Transformation|GetActorLocation _array_element_2) (Transformation|GetActorLocation (Variables|ObjectRefs|GetPlayer))))
          (LocalVariables|SetChosenInteractible _array_element_2)))
      ;[1 0.5277 0 1 34] On interactible select
      (bind _choseninteractible (LocalVariables|GetChosenInteractible)
        (:then
          (if (not (== (Variables|Interactible|GetCurrentlySelectedInteractible) (LocalVariables|GetChosenInteractible))) ; Selected interactible is already the one currently selected - do nothing.
            (bind _output_get (Variables|Interactible|SetCurrentlySelectedInteractible _choseninteractible))
            (Class|BPIInteract|Select(Message) _output_get)))
        (:else
          (bind _currentlyselectedinteractible (Variables|Interactible|GetCurrentlySelectedInteractible)
            (:then
              (Class|BPIInteract|Deselect(Message) _currentlyselectedinteractible)
              (Variables|Interactible|SetCurrentlySelectedInteractible 0))
            (:else)))))
    (:else)))