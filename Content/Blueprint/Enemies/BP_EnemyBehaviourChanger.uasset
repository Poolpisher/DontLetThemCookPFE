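; BP_EnemyBehaviourChanger is a one-shot trigger box that changes the behaviour of registered groom enemies when the player enters it.
; AddGroom builds the list of affected grooms, skipping invalid references and duplicates.
; On the first BP_Player overlap, it calls PickDecision with BehaviourToApply on each valid groom, then destroys itself.
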(event OnComponentBeginOverlap(Box)
  (params (OverlappedComponent :type Primitive%20Component%20Object%20Reference) (OtherActor :type Actor%20Object%20Reference) (OtherComp :type Primitive%20Component%20Object%20Reference) (OtherBodyIndex :type Integer) (bFromSweep :type Boolean) (SweepResult :type Hit%20Result%20Structure%20%28by%20ref%29))
  ;[1 0 0 1 34] Trigger
  (Utilities|Casting|CastToBP_Player OtherActor)
  (Utilities|FlowControl|DoOnce false
    (:Completed
      (for _array_element (Variables|Default|Getgrooms)
        (Utilities|IsValid _array_element
          (:Is%20Valid
            (Default|PickDecision _array_element (Variables|Default|GetbehaviourToApply)))))
      (Actor|DestroyActor))))

(event Custom|AddGroom
  (params (groomToAdd :type BP%20Groom%20Object%20Reference%20%28by%20ref%29))
  ;[0 0 1 1 34] Add groom
  (Utilities|IsValid groomToAdd
    (:Is%20Valid
      (if (not (Utilities|Array|ContainsItem (Variables|Default|Getgrooms) groomToAdd))
        (Utilities|Array|Add (Variables|Default|Getgrooms) groomToAdd)))))

(fn ConstructionScript)