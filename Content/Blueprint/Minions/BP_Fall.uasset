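; BP_Fall is a smart nav link Blueprint that moves minions across a link, named for falls.
; When an agent reaches the link, it casts to BPP_Minions and teleports that minion straight to the link destination without sweeping.
; An unconnected alternative that would launch the minion on a suggested projectile arc toward lower destinations remains in the graph but never runs.
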(event EventSmartLinkReached
  (params (Agent :type Actor%20Object%20Reference) (Destination :type Vector%20%28by%20ref%29 :default "0, 0, 0"))
  (bind _asbpp_minions (Utilities|Casting|CastToBPP_Minions Agent))
  (Transformation|SetActorLocation _asbpp_minions Destination false true))

(fn ConstructionScript)