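; Base interactable actor that child Blueprints extend, with placeholder Select, Deselect, Enable and Disable events.
; Interact switches on InteractionType: Unlimited fires InteractionEvent every time, Do Once fires it once then disables interaction and optionally destroys the actor, and Flip Flop alternates Enable and Disable.
; InteractionEvent prints a debug string and plays an optional sound at the actor.
; Collider overlaps with BP_Player show and animate the W_Interact prompt, then hide it on exit.
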(event OnComponentBeginOverlap(Collider)
  (params (OverlappedComponent :type Primitive%20Component%20Object%20Reference) (OtherActor :type Actor%20Object%20Reference) (OtherComp :type Primitive%20Component%20Object%20Reference) (OtherBodyIndex :type Integer) (bFromSweep :type Boolean) (SweepResult :type Hit%20Result%20Structure%20%28by%20ref%29))
  (bind _widget (Variables|Default|GetWidget))
  ;[0 1 1 1 34] Widget interact
  (Utilities|Casting|CastToBP_Player OtherActor)
  (Development|SetHiddeninGame _widget false false)
  (bind _asw_interact (Utilities|Casting|CastToW_Interact (UserInterface|GetWidget _widget)))
  (Default|PlayAnim _asw_interact))

(event OnComponentEndOverlap(Collider)
  (params (OverlappedComponent :type Primitive%20Component%20Object%20Reference) (OtherActor :type Actor%20Object%20Reference) (OtherComp :type Primitive%20Component%20Object%20Reference) (OtherBodyIndex :type Integer))
  ;[0 1 1 1 34] Widget interact
  (Utilities|Casting|CastToBP_Player OtherActor)
  (Development|SetHiddeninGame (Variables|Default|GetWidget) true false))

(event Custom|Interaction%20Event
  (params (Interactor :type BPC%20Interactor%20Object%20Reference))
  ;[0 0.4 1 1 34] Interact event
  (Development|PrintString "Interact")
  (bind _soundtoplay (Variables|Default|GetsoundToPlay)
    (:then
      (Audio|PlaySoundatLocation _soundtoplay (Transformation|GetActorLocation) "0, 0, 0" 1.0 1.0 0.0 "/Game/Sounds/SA_Main.SA_Main" 0 0 0))
    (:else)))

(event Custom|Disable
  ;[0 0.4 1 1 34] Interact event
  (Development|PrintString "Disable"))

(event Custom|Enable
  ;[0 0.4 1 1 34] Interact event
  (Development|PrintString "Enable"))

(event EventSelect
  ;[1 0.7812 0 1 34] Selection
)

(event EventDeselect
  ;[1 0.7812 0 1 34] Selection
)

(event EventInteract
  (params (Interactor :type BPC%20Interactor%20Object%20Reference))
  ;[0 0 1 1 34] Interaction
  (switch Utilities|FlowControl|Switch|SwitchonEnum_InteractionType (Variables|Parameters|GetinteractionType)
    (:NewEnumerator0
      (CallFunction|InteractionEvent Interactor))
    (:NewEnumerator1
      (Utilities|FlowControl|DoOnce false
        (:Completed
          (CallFunction|InteractionEvent Interactor)
          (Variables|Parameters|SetCanBeInteractedWith? false)
          (if (Variables|Parameters|GetdestroyOnInteract)
            (Actor|DestroyActor)))))
    (:NewEnumerator2
      (Utilities|FlowControl|FlipFlop
        (:A
          (CallFunction|Enable))
        (:B
          (CallFunction|Disable))))))

(fn ConstructionScript)