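; Level-art prop Blueprint for a group of five folders with randomized colors.
; The construction script gives each folder component a material picked independently at random from blue, pink, yellow and green instances, so neighbors can share a color.
; The random pick is unseeded, so colors can change whenever the construction script reruns.
; The event graph has no active logic.
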(event EventBeginPlay)

(event Collision|EventActorBeginOverlap
  (params (OtherActor :type Actor%20Object%20Reference)))

(event EventTick
  (params (DeltaSeconds :type Float%20%28single-precision%29)))

(fn ConstructionScript
  (bind _array (Utilities|Array|MakeArray "/Game/Materials/StaffRoom/MI_Folder_Blue.MI_Folder_Blue" "/Game/Materials/StaffRoom/MI_Folder_Pink.MI_Folder_Pink" "/Game/Materials/StaffRoom/MI_Folder_Yellow.MI_Folder_Yellow" "/Game/Materials/StaffRoom/MI_Folder_Green.MI_Folder_Green"))
  (bind _outitem (Utilities|Array|Random _array))
  (Rendering|Material|SetMaterial (Variables|Default|GetFolder_1) 0 _outitem)
  (Rendering|Material|SetMaterial (Variables|Default|GetFolder_2) 0 _outitem)
  (Rendering|Material|SetMaterial (Variables|Default|GetFolder_3) 0 _outitem)
  (Rendering|Material|SetMaterial (Variables|Default|GetFolder_4) 0 _outitem)
  (Rendering|Material|SetMaterial (Variables|Default|GetFolder_5) 0 _outitem))