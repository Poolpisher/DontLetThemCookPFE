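; BP_Drawer is a drawer level element that alternately pulls out and pushes in, carrying the actor that moves it along.
; MoveDrawer lerps both along the drawer's right vector on a Timeline, then flips the direction.
; Left, Right and Front triggers register drawer and side on BP_Player, and GetSpline returns that side's spline.
; Tick shows an interact widget by player distance while openable, and the construction script picks the visible folder mesh.
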(event OnComponentBeginOverlap(Left)
  (params (OverlappedComponent :type Primitive%20Component%20Object%20Reference) (OtherActor :type Actor%20Object%20Reference) (OtherComp :type Primitive%20Component%20Object%20Reference) (OtherBodyIndex :type Integer) (bFromSweep :type Boolean) (SweepResult :type Hit%20Result%20Structure%20%28by%20ref%29))
  (bind _asbp_player (Utilities|Casting|CastToBP_Player OtherActor))
  (Variables|/Game/Blueprint/Player/BP_Player.BP_Player_C|SetDrawerSide _asbp_player "NewEnumerator2")
  (Variables|/Game/Blueprint/Player/BP_Player.BP_Player_C|SetDrawer _asbp_player self))

(event OnComponentEndOverlap(Left)
  (params (OverlappedComponent :type Primitive%20Component%20Object%20Reference) (OtherActor :type Actor%20Object%20Reference) (OtherComp :type Primitive%20Component%20Object%20Reference) (OtherBodyIndex :type Integer))
  (bind _asbp_player (Utilities|Casting|CastToBP_Player OtherActor))
  (Variables|/Game/Blueprint/Player/BP_Player.BP_Player_C|SetDrawerSide _asbp_player "NewEnumerator3")
  (Variables|/Game/Blueprint/Player/BP_Player.BP_Player_C|SetDrawer _asbp_player 0))

(event OnComponentBeginOverlap(Right)
  (params (OverlappedComponent :type Primitive%20Component%20Object%20Reference) (OtherActor :type Actor%20Object%20Reference) (OtherComp :type Primitive%20Component%20Object%20Reference) (OtherBodyIndex :type Integer) (bFromSweep :type Boolean) (SweepResult :type Hit%20Result%20Structure%20%28by%20ref%29))
  (bind _asbp_player (Utilities|Casting|CastToBP_Player OtherActor))
  (Variables|/Game/Blueprint/Player/BP_Player.BP_Player_C|SetDrawerSide _asbp_player "NewEnumerator1")
  (Variables|/Game/Blueprint/Player/BP_Player.BP_Player_C|SetDrawer _asbp_player self))

(event OnComponentEndOverlap(Right)
  (params (OverlappedComponent :type Primitive%20Component%20Object%20Reference) (OtherActor :type Actor%20Object%20Reference) (OtherComp :type Primitive%20Component%20Object%20Reference) (OtherBodyIndex :type Integer))
  (bind _asbp_player (Utilities|Casting|CastToBP_Player OtherActor))
  (Variables|/Game/Blueprint/Player/BP_Player.BP_Player_C|SetDrawerSide _asbp_player "NewEnumerator3")
  (Variables|/Game/Blueprint/Player/BP_Player.BP_Player_C|SetDrawer _asbp_player 0))

(event OnComponentBeginOverlap(Front)
  (params (OverlappedComponent :type Primitive%20Component%20Object%20Reference) (OtherActor :type Actor%20Object%20Reference) (OtherComp :type Primitive%20Component%20Object%20Reference) (OtherBodyIndex :type Integer) (bFromSweep :type Boolean) (SweepResult :type Hit%20Result%20Structure%20%28by%20ref%29))
  (bind _asbp_player (Utilities|Casting|CastToBP_Player OtherActor))
  (Variables|/Game/Blueprint/Player/BP_Player.BP_Player_C|SetDrawerSide _asbp_player "NewEnumerator0")
  (Variables|/Game/Blueprint/Player/BP_Player.BP_Player_C|SetDrawer _asbp_player self))

(event OnComponentEndOverlap(Front)
  (params (OverlappedComponent :type Primitive%20Component%20Object%20Reference) (OtherActor :type Actor%20Object%20Reference) (OtherComp :type Primitive%20Component%20Object%20Reference) (OtherBodyIndex :type Integer))
  (bind _asbp_player (Utilities|Casting|CastToBP_Player OtherActor))
  (Variables|/Game/Blueprint/Player/BP_Player.BP_Player_C|SetDrawerSide _asbp_player "NewEnumerator3")
  (Variables|/Game/Blueprint/Player/BP_Player.BP_Player_C|SetDrawer _asbp_player 0))

(event Custom|MoveDrawer
  (params (Actor :type Actor%20Object%20Reference))
  (bind _returnvalue (Transformation|GetActorLocation))
  ;[1 1 0 1 34] Move drawer
  (Variables|Default|SetActor Actor)
  (if (not (Variables|Default|GetIsOpening))
    (if (Variables|Default|GetcanOpen)
      (Variables|Default|SetfirstBeetleLoc (Transformation|GetActorLocation (Variables|Default|GetActor)))
      (Variables|Default|SettargetBeetleLoc (+ (Transformation|GetActorLocation (Variables|Default|GetActor)) (* (Transformation|GetActorRightVector) (* (Variables|Default|Getrange) (Utilities|Select :Index (Variables|Default|Getmove) :NewEnumerator1 1.0 :NewEnumerator0 -1.0)))))
      (Variables|Default|SetfirstDrawerLoc _returnvalue)
      (Variables|Default|SettargetLoc (+ _returnvalue (* (Transformation|GetActorRightVector) (* (Variables|Default|Getrange) (Utilities|Select :Index (Variables|Default|Getmove) :NewEnumerator1 1.0 :NewEnumerator0 -1.0)))))
      (Variables|Default|SetIsOpening true)
      (bind _track (Timeline|Timeline PlayFromStart)
        (:Update
          (Transformation|SetActorLocation (Math|Vector|Lerp(Vector) (Variables|Default|GetfirstDrawerLoc) (Variables|Default|GettargetLoc) _track) false true)
          (Transformation|SetActorLocation (Variables|Default|GetActor) (Math|Vector|Lerp(Vector) (Variables|Default|GetfirstBeetleLoc) (Variables|Default|GettargetBeetleLoc) _track) false false))
        (:Finished
          (Variables|Default|Setmove (Utilities|Select :Index (Variables|Default|Getmove) :NewEnumerator1 "NewEnumerator0" :NewEnumerator0 "NewEnumerator1"))
          (Variables|Default|SetIsOpening false))))))

(event Custom|ShowFolder
  (bind _sm_foldertype02 (Variables|Default|GetSM_foldertype02))
  (CallFunction|AddFolder)
  (Utilities|IsValid _sm_foldertype02
    (:Is%20Valid
      (Rendering|SetVisibility _sm_foldertype02 (Variables|Default|GetFolderVisibile) false))))

(event Custom|ShowInteract
  (bind _widget (Variables|Default|GetWidget))
  ;[0 1 1 1 34] Widget interact
  (if (Variables|Default|GetcanOpen)
    (if (< (Math|Vector|Distance(Vector) (Transformation|GetActorLocation) (Transformation|GetActorLocation (Game|Player|GetPlayerPawn 0))) 175.0)
      (Development|SetHiddeninGame _widget false false)
      (if (not (Variables|Default|GetWidgetShowed))
        (bind _asw_interact (Utilities|Casting|CastToW_Interact (UserInterface|GetWidget _widget)))
        (Default|PlayAnim _asw_interact)
        (Variables|Default|SetWidgetShowed true))
      (else
        (Development|SetHiddeninGame _widget true false :!label _label)
        (Variables|Default|SetWidgetShowed false)))
    (else
      (goto _label))))

(event EventBeginPlay
  ;[0 0 0 1 34] Start
  (Components|Timeline|SetPlayRate (Variables|Default|GetTimeline) (Variables|Default|GetmoveRate))
  (CallFunction|ShowFolder))

(event EventTick
  (params (DeltaSeconds :type Float%20%28single-precision%29))
  (CallFunction|ShowInteract))

(fn ConstructionScript
  (bind _sm_foldertype02 (Variables|Default|GetSM_foldertype02))
  (bind _sm_folderytype031 (Variables|Default|GetSM_folderytype031))
  (switch int (Variables|Default|GetChoose_StaticInside)
    (:Default
      (Rendering|SetVisibility _sm_foldertype02 false false :!label _label)
      (Rendering|SetVisibility (Variables|Default|GetSM_foldertype12) true false))
    (:0
      (goto _label))
    (:1
      (Rendering|SetVisibility _sm_folderytype031 false false)
      (Rendering|SetVisibility _sm_foldertype02 true false))
    (:2
      (Rendering|SetVisibility _sm_foldertype02 false false)
      (Rendering|SetVisibility _sm_folderytype031 true false))))

(fn AddFolder
  (Utilities|Array|Add (Variables|Default|GetFolderList) 0)
  (Utilities|Array|Add (Variables|Default|GetFolderList) 0)
  (Utilities|Array|Add (Variables|Default|GetFolderList) 0)
  (Utilities|Array|Add (Variables|Default|GetFolderList) 0)
  (Utilities|Array|Add (Variables|Default|GetFolderList) 0)
  (Utilities|Array|Add (Variables|Default|GetFolderList) 0)
  (Utilities|Array|Add (Variables|Default|GetFolderList) 0)
  (Utilities|Array|Add (Variables|Default|GetFolderList) 0)
  (Utilities|Array|Add (Variables|Default|GetFolderList) 0)
  (Utilities|Array|Add (Variables|Default|GetFolderList) 0)
  (Utilities|Array|Add (Variables|Default|GetFolderList) 0)
  (Utilities|Array|Add (Variables|Default|GetFolderList) 0)
  (Utilities|Array|Add (Variables|Default|GetFolderList) 0)
  (Utilities|Array|Add (Variables|Default|GetFolderList) 0)
  (Utilities|Array|Add (Variables|Default|GetFolderList) 0))

(fn GetSpline
  (params (Side :type E_DrawerSIde%20Enum :default "NewEnumerator3"))
  (return (Utilities|Select :Index Side :NewEnumerator3 0 :NewEnumerator0 (Variables|Default|GetSplineFront) :NewEnumerator1 (Variables|Default|GetSplineRight) :NewEnumerator2 (Variables|Default|GetSplineLeft))))