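; Game camera actor that follows the player along spline rails defined by camera triggers and plays a looping default shake from BeginPlay.
; Each tick it maps player progress on the first trigger's golden path onto its camera trail, blending per-point rotation, offset, FOV, speed and height-follow.
; Without triggers it trails a weighted average of focus objects.
; SetCam briefly speeds interpolation for near-instant snaps; SpawnSpear launches a broom spear.
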(event Custom|SetCam
  ;[0 0 0 1 34] Start
  (Variables|Default|SetautoSetCam true)
  (Utilities|FlowControl|Delay 0.2)
  (Variables|Default|SetautoSetCam false))

(event Custom|SpawnSpear
  (params (EndPos :type Vector))
  (bind _returnvalue (Game|SpawnActorfromClass "/Game/Blueprint/Enemies/BP_BroomSpear.BP_BroomSpear_C" (Transformation|GetWorldTransform (Variables|Default|GetSpearSpawn)) "Undefined" "MultiplyWithRoot" 0 0))
  (Default|SetupSpear _returnvalue (Transformation|GetWorldLocation (Variables|Default|GetSpearSpawn)) EndPos))

(event EventTick
  (params (DeltaSeconds :type Float%20%28single-precision%29))
  ;[0 0 0 1 34] Update
  (CallFunction|HandleCamera))

(event EventBeginPlay
  ;[0 0 0 1 34] Start
  (bind _returnvalue (Class|LegacyCameraShake|StartLegacyCameraShake (Game|GetPlayerCameraManager 0) "/Game/Blueprint/Camera/CS_Default.CS_Default_C" 1.0 "World" "0, 0, 0"))
  (Variables|Default|SetcameraShakeInstance _returnvalue))

(fn ConstructionScript)

(fn HandleCamera
  (bind _targetrot (Variables|TargetValues|GetTargetRot))
  (bind _camera (Variables|Default|GetCamera))
  (bind _targettransitionspeed (Variables|TargetValues|GetTargetTransitionSpeed))
  (bind _camera_2 (Variables|Default|GetCamera))
  (bind _targetxyoffset (Variables|TargetValues|GetTargetXYOffset))
  (bind _targetxyoffset_2 (Variables|TargetValues|GetTargetXYOffset))
  (bind _camera_3 (Variables|Default|GetCamera))
  (bind _camera_4 (Variables|Default|GetCamera))
  (bind _cameraoffset (Variables|Default|GetcameraOffset))
  (bind _targetxyoffset_3 (Variables|TargetValues|GetTargetXYOffset))
  (bind _camera_5 (Variables|Default|GetCamera))
  (bind _camera_6 (Variables|Default|GetCamera))
  (bind _autosetcam (Variables|Default|GetautoSetCam))
  (bind _camera_7 (Variables|Default|GetCamera))
  (bind _returnvalue (Math|Float|SelectFloat 1e+03 _targettransitionspeed _autosetcam))
  (bind (_x _y) (Math|Vector2D|BreakVector2D _targetxyoffset))
  (bind (_x_2 _y_2) (Math|Vector2D|BreakVector2D _targetxyoffset_2))
  (bind (_x_3 _y_3) (Math|Vector2D|BreakVector2D _targetxyoffset_3))
  (if (> (Utilities|Array|Length (Variables|Default|GetCameraTriggers)) 0)
    (CallFunction|SetTargetValues (CallFunction|GetCurrentCameraParameters))
    (if (Variables|Default|GetlookAtPlayer)
      (Transformation|SetWorldRotation _camera_4 (Math|Rotator|FindLookatRotation (Transformation|GetWorldLocation _camera_4) (Transformation|GetActorLocation (Game|GetPlayerCharacter 0))) false false)
      (else
        (Transformation|SetWorldRotation _camera_2 (Math|Interpolation|RInterpTo (Transformation|GetWorldRotation _camera_2) (Math|Rotator|MakeRotator (.roll _targetrot) (+ (.pitch _targetrot) (.y _cameraoffset)) (+ (.yaw _targetrot) (.x _cameraoffset))) (Utilities|Time|GetWorldDeltaSeconds) _returnvalue) false false)))
    (Variables|/Script/Engine.CameraComponent|SetFieldOfView _camera_3 (Math|Interpolation|FInterpTo (Variables|/Script/Engine.CameraComponent|GetFieldOfView _camera_3) (Variables|TargetValues|GetTargetFOV) (Utilities|Time|GetWorldDeltaSeconds) _returnvalue))
    (Variables|Default|SetCurrentXYOffset (Math|Vector2D|MakeVector2D (.x (Math|Interpolation|VInterpTo (Math|Vector|MakeVector (.x (Variables|Default|GetCurrentXYOffset)) (.y (Variables|Default|GetCurrentXYOffset)) 0.0) (Math|Vector|MakeVector _x_3 _y_3 0.0) (Utilities|Time|GetWorldDeltaSeconds) (Math|Float|SelectFloat 1e+03 (Variables|TargetValues|GetTargetTransitionSpeed) (Variables|Default|GetautoSetCam)))) (.y (Math|Interpolation|VInterpTo (Math|Vector|MakeVector (.x (Variables|Default|GetCurrentXYOffset)) (.y (Variables|Default|GetCurrentXYOffset)) 0.0) (Math|Vector|MakeVector _x_3 _y_3 0.0) (Utilities|Time|GetWorldDeltaSeconds) (Math|Float|SelectFloat 1e+03 (Variables|TargetValues|GetTargetTransitionSpeed) (Variables|Default|GetautoSetCam))))))
    (bind _camera_8 (Variables|Default|GetCamera)
      (:then
        (Transformation|SetWorldLocation _camera_8 (Math|Interpolation|VInterpTo (Transformation|GetWorldLocation _camera_8) (+ (+ (Spline|GetLocationatDistanceAlongSpline (Variables|/Game/Blueprint/Camera/BP_CameraTrigger.BP_CameraTrigger_C|GetCameraTrail (Utilities|Array|Get(acopy) (Variables|Default|GetCameraTriggers))) (Variables|Default|GetCurrentSplineDistance) "World") (Math|Vector|MakeVector 0.0 (.x (Variables|Default|GetCurrentXYOffset)) (.y (Variables|Default|GetCurrentXYOffset)))) (Math|Vector|MakeVector 0.0 0.0 (CallFunction|GetCameraHeightChange (Variables|TargetValues|GetTargetPlayerVerticalFollowWeight)))) (Utilities|Time|GetWorldDeltaSeconds) (Math|Float|SelectFloat 1e+03 (Variables|TargetValues|GetTargetTransitionSpeed) (Variables|Default|GetautoSetCam))) false false)
        (bind _asbp_player (Utilities|Casting|CastToBP_Player (Game|GetPlayerCharacter 0)))
        (Variables|/Game/Blueprint/Player/BP_Player.BP_Player_C|SetmoveBasedOnCam _asbp_player (Variables|Default|GetMove%20Player%20Base%20on%20Cam)))
      (:else))
    (else
      (CallFunction|SetTargetValues)
      (Transformation|SetWorldRotation _camera_7 (Math|Interpolation|RInterpTo (Transformation|GetWorldRotation _camera_7) (Variables|TargetValues|GetTargetRot) (Utilities|Time|GetWorldDeltaSeconds) (Math|Float|SelectFloat 1e+03 (Variables|TargetValues|GetTargetTransitionSpeed) (Variables|Default|GetautoSetCam))) false false)
      (Variables|/Script/Engine.CameraComponent|SetFieldOfView _camera_6 (Math|Interpolation|FInterpTo (Variables|/Script/Engine.CameraComponent|GetFieldOfView _camera_6) (Variables|TargetValues|GetTargetFOV) (Utilities|Time|GetWorldDeltaSeconds) (Math|Float|SelectFloat 1e+03 (Variables|TargetValues|GetTargetTransitionSpeed) (Variables|Default|GetautoSetCam))))
      (Variables|Default|SetCurrentXYOffset (Math|Vector2D|MakeVector2D (.x (Math|Interpolation|VInterpTo (Math|Vector|MakeVector (.x (Variables|Default|GetCurrentXYOffset)) (.y (Variables|Default|GetCurrentXYOffset)) 0.0) (Math|Vector|MakeVector _x _y 0.0) (Utilities|Time|GetWorldDeltaSeconds) (Math|Float|SelectFloat 1e+03 (Variables|TargetValues|GetTargetTransitionSpeed) (Variables|Default|GetautoSetCam)))) (.y (Math|Interpolation|VInterpTo (Math|Vector|MakeVector (.x (Variables|Default|GetCurrentXYOffset)) (.y (Variables|Default|GetCurrentXYOffset)) 0.0) (Math|Vector|MakeVector _x _y 0.0) (Utilities|Time|GetWorldDeltaSeconds) (Math|Float|SelectFloat 1e+03 (Variables|TargetValues|GetTargetTransitionSpeed) (Variables|Default|GetautoSetCam))))))
      (bind _averagefocusposition (Focus|GetAverageFocus))
      (Transformation|SetWorldLocation _camera_5 (Math|Interpolation|VInterpTo (Transformation|GetWorldLocation _camera_5) (+ (+ (* (Math|Vector|GetForwardVector _camera) -6e+02) (* (Math|Vector|GetRightVector _camera) _x_2) (* (Math|Vector|GetUpVector _camera) _y_2)) _averagefocusposition) (Utilities|Time|GetWorldDeltaSeconds) (Math|Float|SelectFloat 1e+03 (Variables|TargetValues|GetTargetTransitionSpeed) (Variables|Default|GetautoSetCam))) false false)
      (bind _asbp_player_2 (Utilities|Casting|CastToBP_Player (Game|GetPlayerCharacter 0)))
      (Variables|/Game/Blueprint/Player/BP_Player.BP_Player_C|SetmoveBasedOnCam _asbp_player_2 false))))

(fn AddFocusObject
  (params (Object :type Actor%20Object%20Reference) (Weight :type Integer))
  (Utilities|Array|Add (Variables|Default|GetFocusObjects) (Utilities|Struct|MakeF_FocusObject Object Weight)))

(fn RemoveFocusObject
  (params (Actor :type Actor%20Object%20Reference) (RemoveAllObjectsOfType :type Boolean))
  (bind _focusobjects (Variables|Default|GetFocusObjects))
  (if RemoveAllObjectsOfType
    (for _array_element _focusobjects
      (if (== (.Actor (Utilities|Struct|BreakF_FocusObject _array_element)) Actor)
        (Utilities|Array|RemoveItem _focusobjects _array_element)))
    (else
      (bind _array_element_2 (Utilities|Array|ForEachLoopwithBreak _focusobjects :!label _label)
        (:LoopBody
          (if (== (.Actor (Utilities|Struct|BreakF_FocusObject _array_element_2)) Actor)
            (Utilities|Array|RemoveItem _focusobjects _array_element_2)
            (goto _label Break)))))))

(fn GetAverageFocus
  (if (> (Utilities|Array|Length (Variables|Default|GetFocusObjects)) 0)
    _
    (else
      (Focus|AddFocusObject (Game|GetPlayerCharacter 0) 1)))
  (for _array_element (Variables|Default|GetFocusObjects)
    (for _index (range 0 (.Weight (Utilities|Struct|BreakF_FocusObject _array_element)))
      (LocalVariables|SetAvgFcsPos (+ (LocalVariables|GetAvgFcsPos) (Transformation|GetActorLocation (.Actor (Utilities|Struct|BreakF_FocusObject _array_element)))))
      (Math|Integer|IncrementInt (LocalVariables|GetTotalWeight))))
  (return (/ (LocalVariables|GetAvgFcsPos) (LocalVariables|GetTotalWeight))))

(fn GetCurrentCameraParameters
  (bind _output_get (Variables|Default|SetCurrentSplineDistance (CallFunction|GetCurrentDistanceAlongCurrentSpline)))
  (return (CallFunction|GetBlendedCameraParametersfromDistanceAlongSpline _output_get)))

(fn GetCurrentDistanceAlongCurrentSpline
  (bind _cameratriggers (Variables|Default|GetCameraTriggers))
  (bind _output (Utilities|Array|Get(acopy) _cameratriggers))
  (Utilities|Casting|CastToBP_Player (Game|GetPlayerCharacter 0))
  (if (> (Utilities|Array|Length _cameratriggers) 0)
    (bind _charactergoldenpath (Variables|/Game/Blueprint/Camera/BP_CameraTrigger.BP_CameraTrigger_C|GetCharacterGoldenPath _output)
      (:then
        (bind _cameratrail (Variables|/Game/Blueprint/Camera/BP_CameraTrigger.BP_CameraTrigger_C|GetCameraTrail _output)
          (:then
            (return (Math|Float|Lerp 0.0 (Spline|GetSplineLength _cameratrail) (/ (Class|SplineComponent|GetDistanceAlongSplineatLocation _charactergoldenpath (Transformation|GetActorLocation (Game|GetPlayerCharacter 0)) "World") (Spline|GetSplineLength _charactergoldenpath)))))
          (:else)))
      (:else))))

(fn GetBlendedCameraParametersfromDistanceAlongSpline
  (params (DistanceAlongSpline :type Float%20%28double-precision%29))
  (bind _cameratriggers (Variables|Default|GetCameraTriggers))
  (bind _output (Utilities|Array|Get(acopy) _cameratriggers))
  (bind _cameraparameters (Variables|/Game/Blueprint/Camera/BP_CameraTrigger.BP_CameraTrigger_C|GetCameraParameters _output))
  (bind _cameratrail (Variables|/Game/Blueprint/Camera/BP_CameraTrigger.BP_CameraTrigger_C|GetCameraTrail _output))
  (bind _index (Utilities|FlowControl|ForLoopwithBreak 0 (Spline|GetNumberOfSplinePoints _cameratrail) :!label _label)
    (:LoopBody
      (if (<= (Spline|GetDistanceAlongSplineatSplinePoint _cameratrail _index) DistanceAlongSpline)
        (LocalVariables|SetCurrentIndex _index)
        (else
          (LocalVariables|SetDistanceAtNextPoint (Spline|GetDistanceAlongSplineatSplinePoint _cameratrail _index))
          (goto _label Break))))
    (:Completed
      (LocalVariables|SetCurrentCameraParameters (Utilities|Array|Get(acopy) _cameraparameters (LocalVariables|GetCurrentIndex)))
      (LocalVariables|SetNextCameraParameters (Utilities|Array|Get(acopy) _cameraparameters (+ (LocalVariables|GetCurrentIndex) 1)))
      (LocalVariables|SetAlpha (/ (- (Variables|Default|GetCurrentSplineDistance) (Spline|GetDistanceAlongSplineatSplinePoint (Variables|/Game/Blueprint/Camera/BP_CameraTrigger.BP_CameraTrigger_C|GetCameraTrail _output) (LocalVariables|GetCurrentIndex))) (- (LocalVariables|GetDistanceAtNextPoint) (Spline|GetDistanceAlongSplineatSplinePoint (Variables|/Game/Blueprint/Camera/BP_CameraTrigger.BP_CameraTrigger_C|GetCameraTrail _output) (LocalVariables|GetCurrentIndex)))))
      (return (Utilities|Struct|MakeF_CameraParameters (Math|Rotator|MakeRotator (Math|Float|Lerp (.roll (.BaseRotation (Utilities|Struct|BreakF_CameraParameters (LocalVariables|GetCurrentCameraParameters)))) (.roll (.BaseRotation (Utilities|Struct|BreakF_CameraParameters (LocalVariables|GetNextCameraParameters)))) (LocalVariables|GetAlpha)) (Math|Float|Lerp (.pitch (.BaseRotation (Utilities|Struct|BreakF_CameraParameters (LocalVariables|GetCurrentCameraParameters)))) (.pitch (.BaseRotation (Utilities|Struct|BreakF_CameraParameters (LocalVariables|GetNextCameraParameters)))) (LocalVariables|GetAlpha)) (Math|Float|Lerp (.yaw (.BaseRotation (Utilities|Struct|BreakF_CameraParameters (LocalVariables|GetCurrentCameraParameters)))) (.yaw (.BaseRotation (Utilities|Struct|BreakF_CameraParameters (LocalVariables|GetNextCameraParameters)))) (LocalVariables|GetAlpha))) (Math|Vector2D|MakeVector2D (Math|Float|Lerp (.x (.BaseFocusXYOffset (Utilities|Struct|BreakF_CameraParameters (LocalVariables|GetCurrentCameraParameters)))) (.x (.BaseFocusXYOffset (Utilities|Struct|BreakF_CameraParameters (LocalVariables|GetNextCameraParameters)))) (LocalVariables|GetAlpha)) (Math|Float|Lerp (.y (.BaseFocusXYOffset (Utilities|Struct|BreakF_CameraParameters (LocalVariables|GetCurrentCameraParameters)))) (.y (.BaseFocusXYOffset (Utilities|Struct|BreakF_CameraParameters (LocalVariables|GetNextCameraParameters)))) (LocalVariables|GetAlpha))) (Math|Float|Lerp (.Fieldofview (Utilities|Struct|BreakF_CameraParameters (LocalVariables|GetCurrentCameraParameters))) (.Fieldofview (Utilities|Struct|BreakF_CameraParameters (LocalVariables|GetNextCameraParameters))) (LocalVariables|GetAlpha)) (Math|Float|Lerp (.Transitionspeed (Utilities|Struct|BreakF_CameraParameters (LocalVariables|GetCurrentCameraParameters))) (.Transitionspeed (Utilities|Struct|BreakF_CameraParameters (LocalVariables|GetNextCameraParameters))) (LocalVariables|GetAlpha)) (Math|Float|Lerp (.PlayerVerticalFollowWeight (Utilities|Struct|BreakF_CameraParameters (LocalVariables|GetCurrentCameraParameters))) (.PlayerVerticalFollowWeight (Utilities|Struct|BreakF_CameraParameters (LocalVariables|GetNextCameraParameters))) (LocalVariables|GetAlpha)) (.lookAtPlayer (Utilities|Struct|BreakF_CameraParameters (LocalVariables|GetNextCameraParameters))) (.movePlayerBaseOnCam (Utilities|Struct|BreakF_CameraParameters (LocalVariables|GetNextCameraParameters))))))))

(fn GetCameraHeightChange
  (params (CurrentHeightChangeWeight :type Float%20%28double-precision%29))
  (bind _returnvalue (Game|GetPlayerCharacter 0))
  (bind _cameratriggers (Variables|Default|GetCameraTriggers))
  (bind _returnvalue_2 (Transformation|GetActorLocation _returnvalue))
  (bind _output (Utilities|Array|Get(acopy) _cameratriggers))
  (bind _charactergoldenpath (Variables|/Game/Blueprint/Camera/BP_CameraTrigger.BP_CameraTrigger_C|GetCharacterGoldenPath _output))
  (Utilities|Casting|CastToBP_Player _returnvalue)
  (return (* (- (.Z (Math|Vector|BreakVector _returnvalue_2)) (.Z (Math|Vector|BreakVector (.location (Spline|GetTransformatDistanceAlongSpline _charactergoldenpath (Class|SplineComponent|GetDistanceAlongSplineatLocation _charactergoldenpath _returnvalue_2 "World") "World" false))))) (Math|Float|Clamp(Float) CurrentHeightChangeWeight))))

(fn SetTargetValues
  (params (TargetCameraParams :type F%20Camera%20Parameters%20Structure))
  (bind (_baserotation _basefocusxyoffset _fieldofview _transitionspeed _playerverticalfollowweight _lookatplayer _moveplayerbaseoncam) (Utilities|Struct|BreakF_CameraParameters TargetCameraParams))
  (Variables|TargetValues|SetTargetRot _baserotation)
  (Variables|TargetValues|SetTargetXYOffset _basefocusxyoffset)
  (Variables|TargetValues|SetTargetFOV _fieldofview)
  (Variables|TargetValues|SetTargetTransitionSpeed _transitionspeed)
  (Variables|TargetValues|SetTargetPlayerVerticalFollowWeight _playerverticalfollowweight)
  (Variables|Default|SetlookAtPlayer _lookatplayer)
  (Variables|Default|SetMove%20Player%20Base%20on%20Cam _moveplayerbaseoncam))