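; Cinematic background camera that uses a scene capture component to capture chosen actors from an indexed actor array.
; The construction script adds the components of the actor at the current index to the capture's show-only list, leaving out child actors.
; The SetTarget event stores a new index and adds that actor the same way, without clearing earlier entries.
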(event Custom|SetTarget
  (params (Index :type Integer))
  (bind _output_get (Variables|Default|SetIndex Index))
  (Rendering|SceneCapture|ShowOnlyActorComponents (Variables|Default|GetSceneCaptureComponent2D) (Utilities|Array|Get(acopy) (Variables|Default|GetIn%20Actor) _output_get) false))

(fn ConstructionScript
  (Rendering|SceneCapture|ShowOnlyActorComponents (Variables|Default|GetSceneCaptureComponent2D) (Utilities|Array|Get(acopy) (Variables|Default|GetIn%20Actor) (Variables|Default|GetIndex)) false))