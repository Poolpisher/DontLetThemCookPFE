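; Door level element that opens in a scripted sequence when the player first enters its trigger box, or after a groom trigger and delay.
; The player is locked, attached to the handle and eased into a grip pose at SnackPos.
; Chained timelines turn the handle, swing the door, then release the player and return the handle.
; Each swing flips the door's direction, and the first pops a "Clack" onomatopoeia before destroying it.
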(event OnComponentBeginOverlap(Box)
  (params (OverlappedComponent :type Primitive%20Component%20Object%20Reference) (OtherActor :type Actor%20Object%20Reference) (OtherComp :type Primitive%20Component%20Object%20Reference) (OtherBodyIndex :type Integer) (bFromSweep :type Boolean) (SweepResult :type Hit%20Result%20Structure%20%28by%20ref%29))
  ;[1 0 0 1 34] Trigger
  (bind _asbp_player (Utilities|Casting|CastToBP_Player OtherActor))
  (Variables|Default|SetplayerRef _asbp_player)
  (Utilities|FlowControl|DoOnce false
    (:Completed
      (CallFunction|LockPlayer))))

(event Custom|LockPlayer
  (bind _playerref (Variables|Default|GetplayerRef))
  (bind _mesh (Variables|/Script/Engine.Character|GetMesh _playerref))
  ;[1 1 0 1 34] Lock player to handle
  (Pawn|Components|CharacterMovement|SetMovementMode (Variables|/Script/Engine.Character|GetCharacterMovement (Variables|Default|GetplayerRef)) "MOVE_None" 0)
  (Transformation|AttachComponentToComponent (Variables|Default|GetplayerRef) (Variables|Default|GetHandleInteract) "None" "KeepWorld" "KeepRelative" "KeepRelative" true)
  (CallFunction|MoveHandle "Forward")
  (Utilities|FlowControl|DoOnce false
    (:Completed
      (Utilities|FlowControl|Sequence
        (:then_0
          (Components|Animation|PlayAnimation _mesh "/Game/Blueprint/Player/PLayerTest/Snack_Grip.Snack_Grip" false)
          (Utilities|FlowControl|Delay 2.0)
          (Components|Animation|SetAnimationMode _mesh "AnimationBlueprint" true))
        (:then_1
          (bind _newtrack_0 (Timeline|Timeline Play)
            (:Update
              (Transformation|SetActorLocationAndRotation (Variables|Default|GetplayerRef) (Math|Vector|Lerp(Vector) (Transformation|GetActorLocation (Variables|Default|GetplayerRef)) (Transformation|GetWorldLocation (Variables|Default|GetSnackPos)) _newtrack_0) (Variables|/Script/Engine.SceneComponent|GetRelativeRotation (Variables|Default|GetSnackPos))))))))))

(event Custom|MoveHandle
  (params (direction :type ETimelineDirection%20Enum :default "Forward"))
  (bind _handlerotation (Variables|Default|GethandleRotation))
  ;[1 0.2443 0 1 34] Door moves
  (Utilities|FlowControl|DoOnce false :!label _label
    (:Completed
      (Variables|Default|SetfirstHandleRot (Transformation|GetWorldRotation (Variables|Default|GetHandleInteract)))
      (bind _track (Timeline|Timeline_Handle PlayFromStart)
        (:Update
          (Transformation|SetWorldRotation (Variables|Default|GetHandleInteract) (Math|Rotator|Lerp(Rotator) (Variables|Default|GetfirstHandleRot) (Math|Rotator|MakeRotator (.Roll (Math|Rotator|BreakRotator (Variables|Default|GetfirstHandleRot))) (+ (.Pitch (Math|Rotator|BreakRotator (Variables|Default|GetfirstHandleRot))) (Utilities|Select :Index direction :Forward _handlerotation :Backward (* _handlerotation -1.0))) (.Yaw (Math|Rotator|BreakRotator (Variables|Default|GetfirstHandleRot)))) _track true) false false))
        (:Finished
          (switch Utilities|FlowControl|Switch|SwitchonETimelineDirection direction
            (:Forward
              (CallFunction|OpenDoor)
              (goto _label Reset))
            (:Backward
              (goto _label Reset))))))))

(event Custom|OpenDoor
  (bind _onomatopé (Variables|Default|GetOnomatopé))
  ;[1 0.2443 0 1 34] Door moves
  (Variables|Default|SetfirstDoorRot (Transformation|GetWorldRotation (Variables|Default|GetDoorParent)))
  (bind (_direction _track) (Timeline|Timeline_OpenDoor PlayFromStart)
    (:Update
      (Transformation|SetWorldRotation (Variables|Default|GetDoorParent) (Math|Rotator|Lerp(Rotator) (Variables|Default|GetfirstDoorRot) (|GetWantedDoorRotation) _track true) false false))
    (:Finished
      (switch Utilities|FlowControl|Switch|SwitchonETimelineDirection _direction
        (:Forward
          (bind _playerref (Variables|Default|GetplayerRef)
            (:then
              (Pawn|Components|CharacterMovement|SetMovementMode (Variables|/Script/Engine.Character|GetCharacterMovement _playerref) "MOVE_Walking" 0)
              (Transformation|DetachFromActor (Variables|Default|GetplayerRef) "KeepWorld" "KeepWorld" "KeepWorld"))
            (:else
              _))
          (CallFunction|MoveHandle "Backward")
          (Variables|Default|SetisOpen (not (Variables|Default|GetisOpen)))
          (Variables|Default|SetdoorRotation (* (Variables|Default|GetdoorRotation) -1.0))
          (Utilities|FlowControl|DoOnce false
            (:Completed
              (bind _clack (Timeline|Clack PlayFromStart)
                (:Update
                  (Transformation|SetActorTransform _onomatopé (Math|Transform|MakeTransform (Transformation|GetActorLocation _onomatopé) (Transformation|GetActorRotation _onomatopé) (Math|Vector|MakeVector _clack _clack _clack)) true)
                  (Utilities|FlowControl|Delay 0.4)
                  (Actor|DestroyActor _onomatopé))))))))))

(event EventOnGroomTrigger
  ;[1 0.2443 0 1 34] Door moves
  (Utilities|FlowControl|DoOnce (not (Variables|Default|GetisOpen))
    (:Completed
      (Utilities|FlowControl|Delay (Variables|Default|GetdelayForGroom))
      (CallFunction|MoveHandle "Forward"))))

(event EventBeginPlay
  ;[0 0 0 1 34] Start
  (Components|Timeline|SetPlayRate (Variables|Default|GetTimeline_OpenDoor) (/ (Variables|Default|GetdoorSpeed) 1.0))
  (Components|Timeline|SetPlayRate (Variables|Default|GetTimeline_Handle) (/ (Variables|Default|GethandleSpeed) 1.0)))

(fn ConstructionScript)