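; Rope actor, named for the main menu, built on a cable component with optional yarn ball meshes and proximity-based interact and arrow widgets.
; Construction creates a box collider per cable particle, and BeginPlay tags them "Rope".
; Tick moves, aims and stretches each box toward the next particle, so collision follows the simulated cable.
; Helpers attach or reset the cable end, measure length, and derive direction from the actor's right vector.
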(event Custom|ShowInteract
  (bind _interactwidget (Variables|Default|GetInteractWidget))
  (bind _arrowwidget (Variables|Default|GetArrowWidget))
  ;[0 1 1 1 34] Widget interact
  (Utilities|FlowControl|Sequence
    (:then_0
      (if (Variables|Default|GetisActive)
        (if (< (Math|Vector|Distance(Vector) (Transformation|GetActorLocation) (Transformation|GetActorLocation (Game|Player|GetPlayerPawn 0))) 2e+02)
          (Development|SetHiddeninGame _interactwidget false false)
          (if (not (Variables|Default|GetWidgetShowed))
            (bind _asw_interact (Utilities|Casting|CastToW_Interact (UserInterface|GetWidget _interactwidget)))
            (Default|PlayAnim _asw_interact)
            (Variables|Default|SetWidgetShowed true))
          (else
            (Development|SetHiddeninGame _interactwidget true false :!label _label)
            (Variables|Default|SetWidgetShowed false)))
        (else
          (goto _label))))
    (:then_1
      (if (Variables|Default|GetSpawnArrow)
        (if (Variables|Default|GetisActive)
          (if (< (Math|Vector|Distance(Vector) (Transformation|GetActorLocation) (Transformation|GetActorLocation (Game|Player|GetPlayerPawn 0))) 2e+02)
            (Development|SetHiddeninGame _arrowwidget false false)
            (if (not (Variables|Default|GetWidgetShowed))
              (Utilities|Casting|CastToW_Interact (UserInterface|GetWidget _arrowwidget))
              (Variables|Default|SetWidgetShowed true))
            (else
              (Development|SetHiddeninGame _arrowwidget true false :!label _label_2)
              (Variables|Default|SetWidgetShowed false)))
          (else
            (goto _label_2)))))))

(event Custom|SetDirection
  (bind _cable (Variables|Default|GetCable))
  (bind _locations (Class|CableComponent|GetCableParticleLocations _cable))
  ;[0.0137 0.7379 0.4125 1 34] Direction
  (Variables|Default|Setdirection (select (> (Math|Vector|DotProduct (- (Utilities|Array|Get(acopy) _locations) (Utilities|Array|Get(acopy) _locations (- (Utilities|Array|Length _locations) 1))) (Transformation|GetActorRightVector)) 0.0) "NewEnumerator1" "NewEnumerator0")))

(event Custom|ResetRopeDir
  (Class|CableComponent|SetAttachEndto (Variables|Default|GetCable) (Variables|Default|GetTarget) "None" "None")
  (Variables|/Script/CableComponent.CableComponent|SetEndLocation (Variables|Default|GetCable) "0, 0, 0"))

(event Custom|HideArrow
  ;[0 1 1 1 34] Widget interact
  (Development|SetHiddeninGame (Variables|Default|GetArrowWidget) true false)
  (Variables|Default|SetWidgetShowed false))

(event Custom|SetCableCollisions
  (params (collisionType :type ECollisionEnabled%20Enum :default "NoCollision"))
  ;[0 0.1559 0.1274 1 34] Collisions
  (for _array_element (Variables|Components|Getcollisions)
    (Collision|SetCollisionEnabled _array_element collisionType)))

(event EventTick
  (params (DeltaSeconds :type Float%20%28single-precision%29))
  ;[0 0 0 1 34] Update
  (CallFunction|ShowInteract)
  (for (_array_element _array_index) (Variables|Components|Getcollisions)
    (bind _output_get (Variables|Default|SetCurrentCollision _array_element))
    (Transformation|SetWorldLocation _output_get (Utilities|Array|Get(acopy) (Class|CableComponent|GetCableParticleLocations (Variables|Default|GetCable)) _array_index) false false)
    (if (< _array_index (- (Utilities|Array|Length (Variables|Components|Getcollisions)) 1))
      (Transformation|SetWorldRotation (Variables|Default|GetCurrentCollision) (Math|Rotator|FindLookatRotation (Utilities|Array|Get(acopy) (Class|CableComponent|GetCableParticleLocations (Variables|Default|GetCable)) _array_index) (Utilities|Array|Get(acopy) (Class|CableComponent|GetCableParticleLocations (Variables|Default|GetCable)) (+ _array_index 1))) false false)
      (Components|Box|SetBoxExtent (Variables|Default|GetCurrentCollision) (Math|Vector|MakeVector (/ (Math|Vector|Distance(Vector) (Utilities|Array|Get(acopy) (Class|CableComponent|GetCableParticleLocations (Variables|Default|GetCable)) _array_index) (Utilities|Array|Get(acopy) (Class|CableComponent|GetCableParticleLocations (Variables|Default|GetCable)) (+ _array_index 1))) 1.5) 6.0 6.0) true))))

(event EventBeginPlay
  ;[0 0 0 1 34] Start
  (CallFunction|SetCableAngle)
  (CallFunction|HideArrow)
  (CallFunction|SetDirection)
  (for _array_element (Variables|Components|Getcollisions)
    (Utilities|Array|AddUnique (Variables|/Script/Engine.ActorComponent|GetComponentTags _array_element) "Rope"))
  (if (Variables|Default|GetYarnBallColision)
    (Collision|SetCollisionEnabled (Variables|Default|GetYarnBallMesh) "QueryAndPhysics")))

(fn ConstructionScript
  (Rendering|SetVisibility (Variables|Default|GetYarnBallMesh) (Variables|Default|GetYarnBall_Visibility) false)
  (CallFunction|SetRopeCollision))

(fn GetCableLength
  (bind _cable (Variables|Default|GetCable))
  (bind _locations (Class|CableComponent|GetCableParticleLocations _cable))
  (LocalVariables|SetfirstLoc (Utilities|Array|Get(acopy) _locations))
  (for (_array_element _array_index) _locations
    (if (and (> _array_index 0) (< (+ _array_index 1) (Utilities|Array|Length _locations)))
      (LocalVariables|SetcableLength (+ (LocalVariables|GetcableLength) (Math|Vector|Distance(Vector) (LocalVariables|GetfirstLoc) _array_element)))
      (LocalVariables|SetfirstLoc _array_element)))
  (return (LocalVariables|GetcableLength)))

(fn SetRopeCollision
  (for _array_element (Class|CableComponent|GetCableParticleLocations (Variables|Default|GetCable))
    (bind _returnvalue (AddComponent|AddBoxComponent true (Math|Transform|MakeTransform _array_element "0, 0, 0" "1.000000,1.000000,1.000000")))
    (Utilities|Array|Add (Variables|Components|Getcollisions) _returnvalue))
  (CallFunction|SetCableCollisions "QueryAndPhysics"))

(fn SetCableAngle
  (bind _output_get (Variables|Default|SetLookAtRotation (Math|Rotator|FindLookatRotation (Math|Vector|MakeVector 0.0 0.0 0.0) (Variables|/Script/CableComponent.CableComponent|GetEndLocation (Variables|Default|GetCable)))))
  (Transformation|SetRelativeRotation (Variables|Default|GetRotationScene) _output_get false false))

(fn AttachCable
  (params (Target :type Actor%20Object%20Reference))
  (Utilities|IsValid Target
    (:Is%20Valid
      (Variables|/Script/CableComponent.CableComponent|SetEndLocation (Variables|Default|GetCable) (- (Transformation|GetActorLocation Target) (Transformation|GetActorLocation)))
      (CallFunction|SetCableAngle)
      (Variables|Default|SetTarget Target))
    (:Is%20Not%20Valid
      (Variables|/Script/CableComponent.CableComponent|SetEndLocation (Variables|Default|GetCable) "0, 0, 0")
      (Class|CableComponent|SetAttachEndto (Variables|Default|GetCable) 0 "None" "None"))))