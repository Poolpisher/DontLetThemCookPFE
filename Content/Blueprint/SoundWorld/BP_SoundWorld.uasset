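; BP_SoundWorld is an actor that plays its configured Sound on demand as either a sound effect or music.
; E_PlaySound plays the sound at the actor's location or as 2D audio, depending on the AtLocation flag.
; E_PlayMusic hands the same Sound to GI_Instance's StopAndPlayMusic, delegating music playback to the game instance.
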(event Custom|E_PlaySound
  (if (Variables|Default|GetAtLocation)
    (Audio|PlaySoundatLocation (Variables|Default|GetSound) (Transformation|GetActorLocation) "0, 0, 0" 1.0 1.0 0.0 0 0 0 0)
    (else
      (Audio|PlaySound2D (Variables|Default|GetSound) 1.0 1.0 0.0 0 0))))

(event Custom|E_PlayMusic
  (bind _asgi_instance (Utilities|Casting|CastToGI_Instance (Game|GetGameInstance)))
  (Default|StopandPlayMusic _asgi_instance (Variables|Default|GetSound)))

(fn ConstructionScript)