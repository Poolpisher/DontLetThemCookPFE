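; BP_SeqencePlayer_LobbyPorte is a trigger volume that plays a level sequence, apparently for a lobby door, when the player enters its box.
; On overlap it casts to BP_Player and proceeds only if HasDoorOpen is false and, when NeedKey is set, the player's Keys check passes.
; A DoOnce then creates and plays the sequence player a single time; the player's door and key state are read but never changed here.
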(event OnComponentBeginOverlap(Box)
  (params (OverlappedComponent :type Primitive%20Component%20Object%20Reference) (OtherActor :type Actor%20Object%20Reference) (OtherComp :type Primitive%20Component%20Object%20Reference) (OtherBodyIndex :type Integer) (bFromSweep :type Boolean) (SweepResult :type Hit%20Result%20Structure%20%28by%20ref%29))
  (bind _asbp_player (Utilities|Casting|CastToBP_Player OtherActor))
  (if (not (Variables|/Game/Blueprint/Player/BP_Player.BP_Player_C|GetHas_DoorOpen _asbp_player))
    (if (Variables|Default|GetNeedKey)
      (if (Variables|/Game/Blueprint/Player/BP_Player.BP_Player_C|GetKeys _asbp_player)
        (Utilities|FlowControl|DoOnce false :!label _label
          (:Completed
            (bind _returnvalue (Sequencer|Player|CreateLevelSequencePlayer (Variables|Default|GetLevelSequence) (Utilities|Struct|MakeMovieSceneSequencePlaybackSettings true)))
            (bind _output_get (Variables|Default|SetcurrentLevelSequence _returnvalue))
            (Sequencer|Player|Play _output_get :!class /Script/MovieScene.MovieSceneSequencePlayer))))
      (else
        (goto _label)))))

(fn ConstructionScript)