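; Staff room door actor that locks the player to the door on first contact and can swing open by a set yaw.
; The first player overlap with the box disables character movement and attaches the player to the door.
; A separate OpenDoor event, not called within this graph, rotates the door parent through a timeline lerp.
; The logic to release the player, toggle the open state and reverse the swing is disconnected.
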(event OnComponentBeginOverlap(Box)
  (params (OverlappedComponent :type Primitive%20Component%20Object%20Reference) (OtherActor :type Actor%20Object%20Reference) (OtherComp :type Primitive%20Component%20Object%20Reference) (OtherBodyIndex :type Integer) (bFromSweep :type Boolean) (SweepResult :type Hit%20Result%20Structure%20%28by%20ref%29))
  ;[1 0 0 1 34] Trigger
  (bind _asbp_player (Utilities|Casting|CastToBP_Player OtherActor))
  (Variables|Default|SetplayerRef _asbp_player)
  (Utilities|FlowControl|DoOnce false
    (:Completed
      (CallFunction|LockPlayer))))

(event Custom|LockPlayer
  (bind _playerref (Variables|Default|GetplayerRef))
  ;[1 1 0 1 34] Lock player to handle
  (Pawn|Components|CharacterMovement|SetMovementMode (Variables|/Script/Engine.Character|GetCharacterMovement _playerref) "MOVE_None" 0)
  (Transformation|AttachComponentToComponent _playerref (Variables|Default|GetDoor) "None" "KeepWorld" "KeepRelative" "KeepRelative" true))

(event Custom|OpenDoor
  ;[0 1 0 1 34] Door moves
  (bind _output_get (Variables|Default|SetfirstDoorRot (Transformation|GetWorldRotation (Variables|Default|GetDoorParent))))
  (bind _track (Timeline|Timeline_OpenDoor PlayFromStart)
    (:Update
      (Transformation|SetWorldRotation (Variables|Default|GetDoorParent) (Math|Rotator|Lerp(Rotator) _output_get (Math|Rotator|MakeRotator (.Roll (Math|Rotator|BreakRotator _output_get)) (.Pitch (Math|Rotator|BreakRotator _output_get)) (+ (.Yaw (Math|Rotator|BreakRotator _output_get)) (Variables|Default|GetdoorRotation))) _track true) false false))))

(event EventBeginPlay
  ;[0 0 0 1 34] Start
)

(fn ConstructionScript)