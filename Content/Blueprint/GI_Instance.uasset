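; Game instance that manages background music and provides access to a registered cinematic manager.
; Music changes fade out the current 2D sound and fade in a newly created one, while stopping uses a short delay and clears the reference.
; GetCinematicPlayer returns the stored manager reference, or prints a message if none is valid.
; Init is empty, and a console command to disable screen messages is left unconnected.
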(event Custom|Stop_And_PlayMusic
  (params (Music :type Sound%20Base%20Object%20Reference))
  (Utilities|IsValid (Variables|Default|GetCurrentMusic)
    (:Is%20Valid
      (Audio|Components|Audio|FadeOut (Variables|Default|GetCurrentMusic) (Variables|Default|GetFade%20Duration) 0.0 "Linear" :!class /Script/Engine.AudioComponent)
      (bind _returnvalue (Audio|CreateSound2D Music 1.0 1.0 0.0 0))
      (bind _output_get (Variables|Default|SetCurrentMusic _returnvalue))
      (Audio|Components|Audio|FadeIn _output_get (Variables|Default|GetFade%20Duration) 1.0 0.0 "Linear" :!class /Script/Engine.AudioComponent))
    (:Is%20Not%20Valid
      (bind _returnvalue_2 (Audio|CreateSound2D Music 1.0 1.0 0.0 0))
      (bind _output_get_2 (Variables|Default|SetCurrentMusic _returnvalue_2))
      (Audio|Components|Audio|FadeIn _output_get_2 (Variables|Default|GetFade%20Duration) 1.0 0.0 "Linear" :!class /Script/Engine.AudioComponent))))

(event Custom|StopCurrentMusic
  (Utilities|IsValid (Variables|Default|GetCurrentMusic)
    (:Is%20Valid
      (Audio|Components|Audio|StopDelayed (Variables|Default|GetCurrentMusic) 0.5)
      (Variables|Default|SetCurrentMusic 0))))

(event EventInit)

(fn GetCinematicPlayer
  (bind _cinematicmanagerref (Variables|Default|GetCinematicManagerRef)
    (:then
      (return _cinematicmanagerref))
    (:else
      (Development|PrintString "No cinematic manager registerded!" true true "(R=1.000000,G=0.000000,B=0.000000,A=1.000000)" 5.0))))