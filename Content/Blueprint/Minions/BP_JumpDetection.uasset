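; BP_JumpDetection is a smart nav link handler that moves minions across height differences during navigation.
; When a BPP_Minions agent reaches the link, it compares the destination height with the agent's location.
; For higher destinations the minion jumps, is launched along the scaled offset toward the target, and calls Climb.
; Otherwise it teleports straight to the destination without sweeping.
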(event EventSmartLinkReached
  (params (Agent :type Actor%20Object%20Reference) (Destination :type Vector%20%28by%20ref%29 :default "0, 0, 0"))
  (bind _asbpp_minions (Utilities|Casting|CastToBPP_Minions Agent))
  (if (> (.Z (Math|Vector|BreakVector Destination)) (.Z (Math|Vector|BreakVector (Transformation|GetActorLocation _asbpp_minions))))
    (Character|Jump _asbpp_minions)
    (Character|LaunchCharacter _asbpp_minions (* (- Destination (Transformation|GetActorLocation _asbpp_minions)) 5.0) true true)
    (Default|Climb _asbpp_minions)
    (else
      (Transformation|SetActorLocation _asbpp_minions Destination false true))))

(fn ConstructionScript)