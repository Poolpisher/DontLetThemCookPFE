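; BP_JanitorSpear is a level element that has the player's camera spawn a spear when a BP_Player enters its trigger box.
; The landing position comes from a short vertical Visibility line trace around the Target component, using the impact point.
; If the trace hits nothing, it prints a warning and falls back to the Target's world location.
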(event OnComponentBeginOverlap(Box)
  (params (OverlappedComponent :type Primitive%20Component%20Object%20Reference) (OtherActor :type Actor%20Object%20Reference) (OtherComp :type Primitive%20Component%20Object%20Reference) (OtherBodyIndex :type Integer) (bFromSweep :type Boolean) (SweepResult :type Hit%20Result%20Structure%20%28by%20ref%29))
  (bind _asbp_player (Utilities|Casting|CastToBP_Player OtherActor))
  (bind _impactpoint (CallFunction|GetSpearLandingPosition))
  (Default|SpawnSpear (Variables|/Game/Blueprint/Player/BP_Player.BP_Player_C|Getcamera _asbp_player) _impactpoint))

(fn ConstructionScript)

(fn GetSpearLandingPosition
  (bind _target (Variables|Default|GetTarget))
  (bind _returnvalue (Transformation|GetWorldLocation _target))
  (bind _outhit (Collision|LineTraceByChannel (+ _returnvalue "0.000000,0.000000,25.000000") (- _returnvalue "0.000000,0.000000,100.000000") "TraceTypeQuery1" false 0 "None"))
  (if (.bBlockingHit (Collision|BreakHitResult _outhit))
    (return (.ImpactPoint (Collision|BreakHitResult _outhit)))
    (else
      (Development|PrintString "No impact Point; Spawning spear at TargetLocation" true true "(R=1.000000,G=0.385157,B=0.080674,A=1.000000)" 5.0 "1")
      (return (Transformation|GetWorldLocation (Variables|Default|GetTarget))))))