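; AI Groom character for a chase sequence that idles, patrols a spline path or hunts the player, switching through a behaviour enum.
; Path following starts at the closest spline point, with per-point delays and optional looping.
; PawnSensing triggers the chase, where reaching the player kills them, then the Groom returns to idle.
; While moving states are active, Tick sphere-traces for chase interactables; Slip permanently disables sensing and movement with a camera shake.
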(event OnSeePawn(PawnSensing)
  (params (Pawn :type Pawn%20Object%20Reference))
  ;[1 0.25 0 1 34] Pawn sensing
  (if (Variables|Default|GetcanChase)
    (Utilities|Casting|CastToBP_Player Pawn)
    (CallFunction|PickDecision "NewEnumerator2")))

(event Custom|MoveToNextPoint
  (bind _pathtofollow (Variables|Default|GetpathToFollow))
  (bind _spline (Variables|/Game/Blueprint/Enemies/BP_EnemyPath.BP_EnemyPath_C|GetSpline _pathtofollow))
  (bind _delays (Variables|/Game/Blueprint/Enemies/BP_EnemyPath.BP_EnemyPath_C|Getdelays _pathtofollow))
  ;[0 0 1 1 34] Move
  (Variables|Default|GetpathToFollow
    (:then
      (if (and (>= (Variables|Default|Getindex) 0) (< (Variables|Default|Getindex) (Spline|GetNumberOfSplinePoints (Variables|/Game/Blueprint/Enemies/BP_EnemyPath.BP_EnemyPath_C|GetSpline _pathtofollow))))
        (switch Utilities|FlowControl|Switch|SwitchonEnum_EnemyBehaviour (Variables|Default|GetcurrentBehaviour)
          (:NewEnumerator1
            (AI|AIMoveTo self (Spline|GetLocationatSplinePoint _spline (Variables|Default|Getindex) "World") 0 5.0 true
              (:OnSuccess
                (Utilities|FlowControl|Delay (Math|Float|SelectFloat (Utilities|Array|Get(acopy) _delays (Variables|Default|Getindex)) 0.0 (Utilities|Array|IsValidIndex _delays (Variables|Default|Getindex)))))
              (:OnFail
                _))
            (Variables|Default|Setindex (Math|Integer|SelectInt 0 (+ (Variables|Default|Getindex) 1) (and (>= (Variables|Default|Getindex) (- (Spline|GetNumberOfSplinePoints _spline) 1)) (Variables|Default|GetloopPath))))
            (CallFunction|MovetoNextPoint)))))
    (:else)))

(event Custom|Chase
  (params (target :type Actor%20Object%20Reference))
  ;[1 0 0 1 34] Chase
  (bind _asbp_player (Utilities|Casting|CastToBP_Player target)
    (:then
      (if (not (Variables|/Game/Blueprint/Player/BP_Player.BP_Player_C|GetisDead _asbp_player))
        (Utilities|FlowControl|DoOnce false :!label _label
          (:Completed
            (AI|AIMoveTo self "0, 0, 0" target 5.0 true
              (:OnSuccess
                (if (< (Math|Vector|Distance(Vector) (Transformation|GetActorLocation) (Transformation|GetActorLocation target)) 6e+02)
                  (bind _asbp_player_2 (Utilities|Casting|CastToBP_Player target)
                    (:then
                      (Variables|Default|SethasReachedPlayer true)
                      (Default|Death _asbp_player_2))
                    (:CastFailed
                      _))
                  (Utilities|FlowControl|Delay 1.0)
                  (CallFunction|PickDecision "NewEnumerator0" :!label _label_2)
                  (Utilities|FlowControl|Delay 1.0)
                  (Variables|Default|SethasReachedPlayer false)
                  (goto _label Reset)))
              (:OnFail
                (goto _label_2)))))))
    (:CastFailed
      (goto _label))))

(event Custom|PickDecision
  (params (behaviour :type Enum_EnemyBehaviour%20Enum :default "NewEnumerator0"))
  ;[1 1 0 1 34] Pick decision
  (bind _output_get (Variables|Default|SetcurrentBehaviour behaviour))
  (switch Utilities|FlowControl|Switch|SwitchonEnum_EnemyBehaviour _output_get
    (:NewEnumerator0
      (if (Variables|Default|GetidleAtSpawnPoint)
        (AI|AIMoveTo self (Variables|Default|GetspawnPoint) 0 5.0 true)))
    (:NewEnumerator1
      (Variables|Default|GetpathToFollow
        (:then
          (bind _index (CallFunction|GetClosestLocationPoint))
          (Variables|Default|Setindex _index)
          (CallFunction|MovetoNextPoint))
        (:else)))
    (:NewEnumerator2
      (if (Variables|Default|GetcanChase)
        (CallFunction|Chase (Game|GetPlayerCharacter 0))))))

(event Custom|Slip
  ;[0 1 1 1 34] Slip
  (Variables|Default|SetcanChase false)
  (Components|Movement|StopMovementImmediately (Variables|Character|GetCharacterMovement))
  (Variables|Default|SethasSlipped true)
  (Utilities|FlowControl|Delay 0.6)
  (Class|LegacyCameraShake|StartLegacyCameraShake (Game|GetPlayerCameraManager 0) "/Game/Blueprint/Camera/CS_GroomFall.CS_GroomFall_C" 1.0 "CameraLocal" "0, 0, 0")
  (Components|DestroyComponent (Variables|Default|GetPawnSensing))
  (Utilities|FlowControl|Delay 1.0)
  (Collision|SetCollisionResponsetoChannel (Variables|Character|GetMesh) "ECC_Pawn" "ECR_Block"))

(event EventBeginPlay
  ;[0 0 0 1 34] Start
  (Utilities|FlowControl|Delay (Variables|Default|GetstartDelay))
  (Variables|Default|SetspawnPoint (- (Transformation|GetActorLocation) "0.000000,0.000000,500.000000"))
  (CallFunction|PickDecision (Variables|Default|GetcurrentBehaviour)))

(event EventTick
  (params (DeltaSeconds :type Float%20%28single-precision%29))
  (bind _returnvalue (Transformation|GetActorLocation))
  ;[0 0 0 1 34] Update
  (switch Utilities|FlowControl|Switch|SwitchonEnum_EnemyBehaviour (Variables|Default|GetcurrentBehaviour)
    (:NewEnumerator1
      _)
    (:NewEnumerator2
      _))
  (bind _outhit (Collision|SphereTraceByChannel _returnvalue _returnvalue 4e+02 "TraceTypeQuery1" false 0 "None"))
  (if (and (.bBlockingHit (Collision|BreakHitResult _outhit)) (Utilities|DoesObjectImplementInterface (.HitActor (Collision|BreakHitResult _outhit)) "/Game/Blueprint/LevelElement/BPI_ChaseInteractable.BPI_ChaseInteractable_C"))
    (Class|BPIChaseInteractable|OnGroomTrigger(Message) (.HitActor (Collision|BreakHitResult _outhit)))))

(fn ConstructionScript)

(fn GetClosestLocationPoint
  (bind _pathtofollow (Variables|Default|GetpathToFollow))
  (bind _spline (Variables|/Game/Blueprint/Enemies/BP_EnemyPath.BP_EnemyPath_C|GetSpline _pathtofollow))
  (LocalVariables|SetlastDistance 999999999999.0)
  (for _index (range 0 (- (Spline|GetNumberOfSplinePoints _spline) 1))
    (if (< (Math|Vector|Distance(Vector) (Spline|GetLocationatSplinePoint _spline _index "World") (Transformation|GetActorLocation)) (LocalVariables|GetlastDistance))
      (LocalVariables|SetlastDistance (Math|Vector|Distance(Vector) (Spline|GetLocationatSplinePoint _spline _index "World") (Transformation|GetActorLocation)))
      (LocalVariables|SetclosestIndex _index)))
  (return (LocalVariables|GetclosestIndex)))