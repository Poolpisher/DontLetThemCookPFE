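; Beetle minion Blueprint whose Interact action smashes destructible elements or moves drawers, extending parent minion behaviour.
; It AI-moves to the nearest in-range intact destructible and explodes it along its forward vector, otherwise heads to the nearest drawer's BettyTarget and calls MoveDrawer.
; Interacting again, finishing an explosion, failing a move or finding no target calls PickDecision and clears the interacting flag.
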(event EventBeginPlay
  ;[0 0 0 1 34] Start
  (|CallParentFunction))

(event EventTick
  (params (DeltaSeconds :type Float%20%28single-precision%29))
  ;[0 0 0 1 34] Update
  (|CallParentFunction DeltaSeconds))

(event EventInteract
  (bind _self self)
  ;[0 0 1 1 34] Interact
  (|CallParentFunction)
  (if (Variables|Default|GetisInteracting)
    (CallFunction|PickDecision "NewEnumerator0" :!label _label)
    (Variables|Default|SetisInteracting false)
    (else
      (bind _outactors (Actor|GetAllActorsOfClass "/Game/Blueprint/LevelElement/BP_DestructibleElement.BP_DestructibleElement_C"))
      (if (> (Utilities|Array|Length _outactors) 0)
        (bind _destructible (CallFunction|GetClosestDestructible _outactors))
        (Utilities|IsValid _destructible
          (:Is%20Valid
            (AI|AIMoveTo self "0, 0, 0" _destructible 5.0 true
              (:then
                (Variables|Default|SetisInteracting true))
              (:OnSuccess
                (Default|Explode _destructible (Transformation|GetActorForwardVector))
                (goto _label))
              (:OnFail
                (goto _label))))
          (:Is%20Not%20Valid
            (bind _outactors_2 (Actor|GetAllActorsOfClass "/Game/Blueprint/LevelElement/BP_Drawer.BP_Drawer_C" :!label _label_2))
            (if (> (Utilities|Array|Length _outactors_2) 0)
              (bind _drawer (CallFunction|GetClosestDrawer _outactors_2))
              (Utilities|IsValid _drawer
                (:Is%20Valid
                  (AI|AIMoveTo _self (Transformation|GetWorldLocation (Variables|/Game/Blueprint/LevelElement/BP_Drawer.BP_Drawer_C|GetBettyTarget _drawer)) 0 2e+01 true
                    (:OnSuccess
                      (Default|MoveDrawer _drawer _self)
                      (Variables|Default|SetisInteracting true))
                    (:OnFail
                      (goto _label))))
                (:Is%20Not%20Valid
                  (goto _label)))
              (else
                (goto _label)))))
        (else
          (goto _label_2))))))

(fn ConstructionScript
  (|CallParentFunction))

(fn GetClosestDestructible
  (params (pointsArray :type Array%20of%20BP%20Destructible%20Element%20Object%20References))
  (LocalVariables|SetlastDistance 1e+17)
  (for _array_element pointsArray
    (LocalVariables|SetCheckElement _array_element)
    (if (Math|Boolean|ANDBoolean (< (Math|Vector|Distance(Vector) (Transformation|GetActorLocation _array_element) (Transformation|GetActorLocation)) (LocalVariables|GetlastDistance)) (< (Math|Vector|Distance(Vector) (Transformation|GetActorLocation _array_element) (Transformation|GetActorLocation)) 1.4e+03) (not (Variables|/Game/Blueprint/LevelElement/BP_DestructibleElement.BP_DestructibleElement_C|GethasBeenDestroyed (LocalVariables|GetCheckElement))))
      (LocalVariables|SetlastDistance (Math|Vector|Distance(Vector) (Transformation|GetActorLocation _array_element) (Transformation|GetActorLocation)))
      (LocalVariables|SetClosestPoint (LocalVariables|GetCheckElement))))
  (return (LocalVariables|GetClosestPoint)))

(fn GetToad
  (bind _outactors (Actor|GetAllActorsOfClass "/Game/Blueprint/Minions/BP_MinionToad.BP_MinionToad_C"))
  (if (> (Utilities|Array|Length _outactors) 0)
    (return (Utilities|Array|Get(acopy) _outactors))))

(fn GetClosestDrawer
  (params (pointsArray :type Array%20of%20BP%20Drawer%20Object%20References))
  (LocalVariables|SetlastDistance 1e+17)
  (for _array_element pointsArray
    (if (and (< (Math|Vector|Distance(Vector) (Transformation|GetActorLocation _array_element) (Transformation|GetActorLocation)) (LocalVariables|GetlastDistance)) (< (Math|Vector|Distance(Vector) (Transformation|GetActorLocation _array_element) (Transformation|GetActorLocation)) 1.4e+03))
      (LocalVariables|SetlastDistance (Math|Vector|Distance(Vector) (Transformation|GetActorLocation _array_element) (Transformation|GetActorLocation)))
      (LocalVariables|SetclosestPoint _array_element)))
  (return (LocalVariables|GetclosestPoint)))