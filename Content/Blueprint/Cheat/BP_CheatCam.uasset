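; Free-flying cheat camera pawn that can view through level CineCameraActors and drag the player character along in noclip.
; Enhanced Input, mapped while possessed, feeds Tick-driven movement along control rotation, with a run boost and fixed per-frame vertical steps.
; When CheatWidget's Noclip is on, Tick teleports its DefaultCharacter to the freecam's TargetLoc.
; BeginPlay adds boxes to cine cameras; clicking one switches view, Escape returns, and H toggles the widget.
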(event Input|EnhancedActionEvents|EnhancedInputActionIA_Move
  (params (ActionValue :type Vector%202D%20Structure) (ElapsedSeconds :type Float%20%28double-precision%29) (TriggeredSeconds :type Float%20%28double-precision%29) (InputAction :type Input%20Action%20Object%20Reference :default "/Game/Input/Actions/IA_Move.IA_Move"))
  ;[0 0 1 1 34] Move/Look
  (:Triggered
    (Variables|Default|SetMoveInput ActionValue))
  (:Completed
    (Variables|Default|SetMoveInput "")))

(event Input|EnhancedActionEvents|EnhancedInputActionIA_Look
  (params (ActionValue :type Vector%202D%20Structure) (ElapsedSeconds :type Float%20%28double-precision%29) (TriggeredSeconds :type Float%20%28double-precision%29) (InputAction :type Input%20Action%20Object%20Reference :default "/Game/Input/Actions/IA_Look.IA_Look"))
  ;[0 0 1 1 34] Move/Look
  (:Triggered
    (Variables|Default|SetLookInput ActionValue)
    (Pawn|Input|AddControllerYawInput (.X (Math|Vector2D|BreakVector2D (Variables|Default|GetLookInput))))
    (Pawn|Input|AddControllerPitchInput (* (.Y (Math|Vector2D|BreakVector2D (Variables|Default|GetLookInput))) -1.0)))
  (:Completed
    (Variables|Default|SetLookInput "")))

(event Input|EnhancedActionEvents|EnhancedInputActionIA_Run
  (params (ActionValue :type Boolean) (ElapsedSeconds :type Float%20%28double-precision%29) (TriggeredSeconds :type Float%20%28double-precision%29) (InputAction :type Input%20Action%20Object%20Reference :default "/Game/Input/Actions/IA_Run.IA_Run"))
  ;[0 1 0 1 34] Speed
  (:Started
    (Variables|Default|SetMovementSpeed (* (Variables|Default|GetMovementSpeed) 3.0)))
  (:Completed
    (Variables|Default|SetMovementSpeed (/ (Variables|Default|GetMovementSpeed) 3.0))))

(event Input|EnhancedActionEvents|EnhancedInputActionIA_Jump
  (params (ActionValue :type Boolean) (ElapsedSeconds :type Float%20%28double-precision%29) (TriggeredSeconds :type Float%20%28double-precision%29) (InputAction :type Input%20Action%20Object%20Reference :default "/Game/Input/Actions/IA_Jump.IA_Jump"))
  ;[0 0.2 0 1 34] Up/Down
  (:Started
    (Variables|Default|SetV-Type 1))
  (:Completed
    (Variables|Default|SetV-Type 0)))

(event Input|EnhancedActionEvents|EnhancedInputActionIA_Crouch
  (params (ActionValue :type Boolean) (ElapsedSeconds :type Float%20%28double-precision%29) (TriggeredSeconds :type Float%20%28double-precision%29) (InputAction :type Input%20Action%20Object%20Reference :default "/Game/Input/Actions/IA_Crouch.IA_Crouch"))
  ;[0 0.2 0 1 34] Up/Down
  (:Started
    (Variables|Default|SetV-Type 2))
  (:Completed
    (Variables|Default|SetV-Type 0)))

(event EventBeginPlay
  ;[0 0 0 1 34] Start
  (bind _outactors (Actor|GetAllActorsOfClass "/Script/CinematicCamera.CineCameraActor"))
  (for _array_element _outactors
    (Utilities|IsValid (Actor|GetComponentbyClass _array_element "/Script/Engine.BoxComponent")
      (:Is%20Not%20Valid
        (AddComponent|AddBoxComponent _array_element false)))))

(event EventPossessed
  (params (NewController :type Controller%20Object%20Reference))
  ;[1 0 0 1 34] Possessed/Unpossessed
  (CallFunction|SetupInput NewController "/Game/Input/IMC_Cheat.IMC_Cheat")
  (Actor|Tick|SetActorTickEnabled true))

(event EventUnpossessed
  (params (OldController :type Controller%20Object%20Reference))
  ;[1 0 0 1 34] Possessed/Unpossessed
  (Utilities|IsValid OldController
    (:Is%20Valid
      (bind _asplayer_controller (Utilities|Casting|CastToPlayerController OldController))
      (Input|RemoveMappingContext (PlayerController|LocalPlayerSubsystems|GetEnhancedInputLocalPlayerSubsystem _asplayer_controller) "/Game/Input/IMC_Cheat.IMC_Cheat" "(bIgnoreAllPressedKeysUntilRelease=True,bForceImmediately=False,bNotifyUserSettings=False)")
      (Actor|Tick|SetActorTickEnabled false)
      (Variables|Default|SetMoveInput "")
      (Variables|Default|SetLookInput ""))))

(event EventTick
  (params (DeltaSeconds :type Float%20%28single-precision%29))
  (bind _cheatwidget (Variables|Default|GetcheatWidget))
  (bind _freecamref (Variables|/Game/Widgets/Menu/W_Cheat.W_Cheat_C|GetFreecamRef _cheatwidget))
  (bind (_loc _rot) (CallFunction|GetTargetLocandRot _freecamref))
  ;[0 0 0 1 34] Update
  (Transformation|SetActorLocationAndRotation (+ (CallFunction|GetNewLocation DeltaSeconds) (* (Math|Vector|VectorUp) (* (Utilities|Select :Index (Variables|Default|GetV-Type) :Option%200 0.0 :Option%201 1.0 :Option%202 -1.0) 1e+01))) (Pawn|GetControlRotation :!class /Script/Engine.Pawn))
  (if (Variables|/Game/Widgets/Menu/W_Cheat.W_Cheat_C|GetNoclip _cheatwidget)
    (Transformation|SetActorLocationAndRotation (Variables|/Game/Widgets/Menu/W_Cheat.W_Cheat_C|GetDefaultCharacter _cheatwidget) _loc _rot false true)))

(event Input|KeyboardEvents|H
  (params (Key :type Key%20Structure :default "None"))
  (bind _cheatwidget (Variables|Default|GetcheatWidget))
  ;[0 1 1 1 34] Show/Hide menu
  (:Pressed
    (Utilities|FlowControl|FlipFlop
      (:A
        (Widget|SetVisibility _cheatwidget "Hidden"))
      (:B
        (Widget|SetVisibility _cheatwidget "Visible")))))

(event Input|MouseEvents|LeftMouseButton
  (params (Key :type Key%20Structure :default "None"))
  ;[1 1 0 1 34] Possess cine cam
  (:Pressed
    (Variables|Default|GetcurrentCineCam
      (:then)
      (:else
        (bind _ascine_camera_actor (Utilities|Casting|CastToCineCameraActor (.HitActor (Collision|BreakHitResult (.HitResult (Game|Player|GetHitResultUnderCursorbyChannel (Game|GetPlayerController 0) "TraceTypeQuery1" true))))))
        (bind _output_get (Variables|Default|SetcurrentCineCam _ascine_camera_actor))
        (Game|Player|SetViewTargetwithBlend (Game|GetPlayerController 0) _output_get 0.0 "VTBlend_Linear" 0.0 false)))))

(event Input|KeyboardEvents|Escape
  (params (Key :type Key%20Structure :default "None"))
  ;[1 1 0 1 34] Possess cine cam
  (:Pressed
    (Variables|Default|GetcurrentCineCam
      (:then
        (Game|Player|SetViewTargetwithBlend (Game|GetPlayerController 0) self 0.0 "VTBlend_Linear" 0.0 false)
        (Variables|Default|SetcurrentCineCam 0))
      (:else))))

(fn ConstructionScript)

(fn SetupInput
  (params (Controller :type Object%20Object%20Reference) (MappingContext :type Input%20Mapping%20Context%20Object%20Reference))
  ;[1 1 1] This function sets up the character controller to use the Enhanced Input System, which requires a mapping context to be added upon possession.
  (Utilities|IsValid Controller
    (:Is%20Valid
      (bind _asplayer_controller (Utilities|Casting|CastToPlayerController Controller))
      (Input|AddMappingContext (PlayerController|LocalPlayerSubsystems|GetEnhancedInputLocalPlayerSubsystem _asplayer_controller) MappingContext 0 "(bIgnoreAllPressedKeysUntilRelease=True,bForceImmediately=False,bNotifyUserSettings=False)"))))

(fn GetInputDirections
  (bind _returnvalue (Pawn|GetControlRotation :!class /Script/Engine.Pawn))
  (return (Math|Vector|GetRightVector (Math|Rotator|MakeRotator 0.0 0.0 (.yaw _returnvalue))) (Math|Vector|GetForwardVector (Math|Rotator|MakeRotator 0.0 (.pitch _returnvalue) (.yaw _returnvalue)))))

(fn GetNewLocation
  (params (DeltaTime :type Float%20%28double-precision%29))
  (bind (_right _forward) (CallFunction|GetInputDirections))
  (bind _moveinput (Variables|Default|GetMoveInput))
  (bind _movementspeed (Variables|Default|GetMovementSpeed))
  (bind (_x _y) (Math|Vector2D|BreakVector2D _moveinput))
  (bind _returnvalue (* DeltaTime _movementspeed))
  (return (+ (Transformation|GetActorLocation) (+ (* (* _right _x) _returnvalue) (* (* _forward _y) _returnvalue)))))

(fn GetTargetLocandRot
  (bind _targetloc (Variables|Default|GetTargetLoc))
  (return (Transformation|GetWorldLocation _targetloc) (Transformation|GetWorldRotation _targetloc)))