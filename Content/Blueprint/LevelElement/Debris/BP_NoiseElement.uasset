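; Noisy debris prop (toy ball, mouse or balloon) that launches a broom spear when the player steps on it.
; Box overlap spawns and attaches BP_BroomSpear aimed at Target, with Niagara effects and a per-type sound.
; With MoveOnX, a shared timeline rolls the ball or squashes other props, then re-arms after a delay.
; Non-ball balloons also shrink and destroy themselves; the landing-trace helper is not called here.
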(event OnComponentBeginOverlap(Box)
  (params (OverlappedComponent :type Primitive%20Component%20Object%20Reference) (OtherActor :type Actor%20Object%20Reference) (OtherComp :type Primitive%20Component%20Object%20Reference) (OtherBodyIndex :type Integer) (bFromSweep :type Boolean) (SweepResult :type Hit%20Result%20Structure%20%28by%20ref%29))
  (if (Variables|Default|GetCanKill)
    (Utilities|Casting|CastToBP_Player OtherActor)
    (Variables|Default|SetCanKill false)
    (Utilities|FlowControl|Sequence
      (:then_0
        ;[1 1 1] Broom Javelot
        (bind _returnvalue (Game|SpawnActorfromClass "/Game/Blueprint/Enemies/BP_BroomSpear.BP_BroomSpear_C" (Variables|Default|GetTransform_SpawnBroom) "Undefined" "MultiplyWithRoot" 0 0))
        (Transformation|AttachActorToActor _returnvalue self "None" "KeepRelative" "KeepRelative" "KeepRelative" true)
        (Default|SetupSpear _returnvalue (Transformation|GetWorldLocation (Variables|Default|GetTarget)) false))
      (:then_1
        ;[1 1 1] Movement On X
        (if (Variables|Default|GetMoveOnX)
          (Variables|Default|SetInit_Rotate (Transformation|GetWorldRotation (Variables|Default|GetSM)))
          (if (Variables|Default|GetIs_ToyBoule)
            (Variables|Default|SetDegreeRoll 9e+01)
            (Variables|Default|SetInit_Loc_or_Scale (Transformation|GetWorldLocation (Variables|Default|GetSM)))
            (bind _alpha (Timeline|Move_Static PlayFromStart)
              (:Update
                (if (Variables|Default|GetIs_ToyBoule)
                  (Transformation|SetWorldRotation (Variables|Default|GetSM) (Math|Rotator|Lerp(Rotator) (Math|Rotator|MakeRotator (.roll (Variables|Default|GetInit_Rotate)) (.pitch (Variables|Default|GetInit_Rotate)) (.yaw (Variables|Default|GetInit_Rotate))) (Math|Rotator|MakeRotator (+ (.roll (Variables|Default|GetInit_Rotate)) (Variables|Default|GetDegreeRoll)) (.pitch (Variables|Default|GetInit_Rotate)) (.yaw (Variables|Default|GetInit_Rotate))) _alpha) false false)
                  (Transformation|SetWorldLocation (Variables|Default|GetSM) (Math|Vector|Lerp(Vector) (Math|Vector|MakeVector (.x (Variables|Default|GetInit_Loc_or_Scale)) (.y (Variables|Default|GetInit_Loc_or_Scale)) (.z (Variables|Default|GetInit_Loc_or_Scale))) (Math|Vector|MakeVector (- (.x (Variables|Default|GetInit_Loc_or_Scale)) 25.0) (- (.y (Variables|Default|GetInit_Loc_or_Scale)) 5.0) (.z (Variables|Default|GetInit_Loc_or_Scale))) _alpha) false false)
                  (else
                    (Transformation|SetWorldScale3D (Variables|Default|GetSM) (Math|Vector|Lerp(Vector) (Math|Vector|MakeVector (.x (Variables|Default|GetInit_Loc_or_Scale)) (.y (Variables|Default|GetInit_Loc_or_Scale)) (.z (Variables|Default|GetInit_Loc_or_Scale))) (Math|Vector|MakeVector (.x (Variables|Default|GetInit_Loc_or_Scale)) (.y (Variables|Default|GetInit_Loc_or_Scale)) 0.5) _alpha)))))
              (:Finished
                ;[1 1 1] Reset
                (Utilities|FlowControl|Delay (Variables|Default|GetDuration))
                (Variables|Default|SetCanKill true)))
            (else
              (Variables|Default|SetDegreeRoll 45.0)
              (Variables|Default|SetInit_Loc_or_Scale (Transformation|GetWorldScale (Variables|Default|GetSM)))
              (Timeline|Move_Static PlayFromStart)))))
      (:then_2
        ;[1 1 1] Niagara
        ;;[1 1 1] Balloon
        (if (Variables|Default|GetBalloon)
          (Niagara|SpawnSystematLocation "/Game/VFX/ballon_explosion/N_ballon_explosion_01.N_ballon_explosion_01" (Transformation|GetActorLocation)))
        (Niagara|SpawnSystematLocation "/Game/VFX/grelolots/N_grelolots_once.N_grelolots_once" (Transformation|GetActorLocation)))
      (:then_3
        ;[1 1 1] Sound
        (if (Variables|Default|GetIs_ToyBoule)
          (Audio|PlaySoundatLocation (Variables|Sound|GetSound_Ball) (Transformation|GetActorLocation) "0, 0, 0" 1.0 1.0 0.0 0 0 0 0)
          (elif (Variables|Default|GetBalloon)
            ;;[1 1 1] Balloon
            (Audio|PlaySoundatLocation (Variables|Sound|GetSound_Balloon) (Transformation|GetActorLocation) "0, 0, 0" 1.0 1.0 0.0 0 0 0 0)
            (Variables|Default|SetInit_Loc_or_Scale (Transformation|GetWorldScale (Variables|Default|GetSM)))
            (bind _alpha_2 (Timeline|Timeline_0 PlayFromStart)
              (:Update
                (Transformation|SetWorldScale3D (Variables|Default|GetSM) (Math|Vector|Lerp(Vector) (Variables|Default|GetInit_Loc_or_Scale) "0, 0, 0" _alpha_2)))
              (:Finished
                (Actor|DestroyActor)))
            (else
              (Audio|PlaySoundatLocation (Variables|Sound|GetSound_Mouse) (Transformation|GetActorLocation) "0, 0, 0" 1.0 1.0 0.0 0 0 0 0))))))))

(fn ConstructionScript
  (if (Variables|Default|GetIs_ToyBoule)
    (Components|StaticMesh|SetStaticMesh (Variables|Default|GetSM) "/Game/Models/Meshes/StaffRoom/cat_toy_ball.cat_toy_ball")))

(fn GetSpearLandingPosition
  (bind _target (Variables|Default|GetTarget))
  (bind _returnvalue (Transformation|GetWorldLocation _target))
  (bind _outhit (Collision|LineTraceByChannel (+ _returnvalue "0.000000,0.000000,25.000000") (- _returnvalue "0.000000,0.000000,100.000000") "TraceTypeQuery1" false 0 "None"))
  (if (.bBlockingHit (Collision|BreakHitResult _outhit))
    (return (.ImpactPoint (Collision|BreakHitResult _outhit)))
    (else
      (Development|PrintString "No impact Point; Spawning spear at TargetLocation" true true "(R=1.000000,G=0.385157,B=0.080674,A=1.000000)" 5.0 "1")
      (return (Transformation|GetWorldLocation (Variables|Default|GetTarget))))))