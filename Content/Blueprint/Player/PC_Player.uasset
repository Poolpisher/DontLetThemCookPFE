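; Player controller that switches Enhanced Input between gameplay and UI mapping contexts and drives menu navigation.
; UI actions for accept, back, pause, tab and directional moves are routed to BPC_HUD functions according to its current menu state.
; Any key press or release has the HUD refresh its input state, then shows the cursor only for one controller type outside gameplay.
; Tick prints the IsUI flag as debug output.
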(event Custom|SetMappingUI
  (IMC|MappingContextRemove "/Game/Input/IMC_Player.IMC_Player")
  (IMC|MappingContextAdd "/Game/Input/IMC_UI.IMC_UI")
  (Variables|Default|SetIsUI true))

(event Custom|SetMappingGP
  (IMC|MappingContextAdd "/Game/Input/IMC_Player.IMC_Player")
  (IMC|MappingContextRemove "/Game/Input/IMC_UI.IMC_UI")
  (Input|SetInputModeGameOnly self false)
  (Variables|Default|SetIsUI false)
  (Variables|Default|SetbShowMouseCursor false))

(event Input|EnhancedActionEvents|EnhancedInputActionIA_UI_TabNav
  (params (ActionValue :type Float%20%28double-precision%29) (ElapsedSeconds :type Float%20%28double-precision%29) (TriggeredSeconds :type Float%20%28double-precision%29) (InputAction :type Input%20Action%20Object%20Reference :default "/Game/Input/Actions/IA_UI_TabNav.IA_UI_TabNav"))
  (:Started
    (Actions|ChangeTab ActionValue)))

(event Input|EnhancedActionEvents|EnhancedInputActionIA_Pause
  (params (ActionValue :type Boolean) (ElapsedSeconds :type Float%20%28double-precision%29) (TriggeredSeconds :type Float%20%28double-precision%29) (InputAction :type Input%20Action%20Object%20Reference :default "/Game/Input/Actions/IA_Pause.IA_Pause"))
  (:Started
    (CallFunction|SetMappingUI)
    (Default|OpenPauseMenu (Variables|Default|GetHUD))))

(event Input|EnhancedActionEvents|EnhancedInputActionIA_UI_Vertical
  (params (ActionValue :type Float%20%28double-precision%29) (ElapsedSeconds :type Float%20%28double-precision%29) (TriggeredSeconds :type Float%20%28double-precision%29) (InputAction :type Input%20Action%20Object%20Reference :default "/Game/Input/Actions/IA_UI_Vertical.IA_UI_Vertical"))
  (:Started
    (Actions|VerticalMove ActionValue)))

(event Input|EnhancedActionEvents|EnhancedInputActionIA_UI_Horizontal
  (params (ActionValue :type Float%20%28double-precision%29) (ElapsedSeconds :type Float%20%28double-precision%29) (TriggeredSeconds :type Float%20%28double-precision%29) (InputAction :type Input%20Action%20Object%20Reference :default "/Game/Input/Actions/IA_UI_Horizontal.IA_UI_Horizontal"))
  (:Started
    (Actions|HorizontalMove ActionValue)))

(event Input|EnhancedActionEvents|EnhancedInputActionIA_UI_Back
  (params (ActionValue :type Boolean) (ElapsedSeconds :type Float%20%28double-precision%29) (TriggeredSeconds :type Float%20%28double-precision%29) (InputAction :type Input%20Action%20Object%20Reference :default "/Game/Input/Actions/IA_UI_Back.IA_UI_Back"))
  (:Started
    (Actions|Back)))

(event Input|EnhancedActionEvents|EnhancedInputActionIA_UI_Accept
  (params (ActionValue :type Boolean) (ElapsedSeconds :type Float%20%28double-precision%29) (TriggeredSeconds :type Float%20%28double-precision%29) (InputAction :type Input%20Action%20Object%20Reference :default "/Game/Input/Actions/IA_UI_Accept.IA_UI_Accept"))
  (:Started
    (Actions|Accept)))

(event Input|EnhancedActionEvents|EnhancedInputActionIA_UI_Pause
  (params (ActionValue :type Boolean) (ElapsedSeconds :type Float%20%28double-precision%29) (TriggeredSeconds :type Float%20%28double-precision%29) (InputAction :type Input%20Action%20Object%20Reference :default "/Game/Input/Actions/IA_UI_Pause.IA_UI_Pause"))
  (:Started
    (Actions|ClosePause)))

(event EventTick
  (params (DeltaSeconds :type Float%20%28single-precision%29))
  (Development|PrintString (Utilities|String|ToString(Boolean) (Variables|Default|GetIsUI))))

(event EventBeginPlay
  ;[0 0 0] Set Player Ref
  (bind _asbp_player (Utilities|Casting|CastToBP_Player (Game|GetPlayerCharacter 0)))
  (Variables|Default|SetAs%20BP%20Player _asbp_player)
  ;[0 0 0] Set HUD Ref
  (bind _asbpc_hud (Utilities|Casting|CastToBPC_HUD (HUD|GetHUD)))
  (Variables|Default|SetHUD _asbpc_hud))

(event Input|KeyboardEvents|AnyKey
  (params (Key :type Key%20Structure :default "None"))
  (:Pressed
    (Default|SetInputs (Variables|Default|GetHUD) :!label _label)
    (CallFunction|ShowMouse))
  (:Released
    (goto _label)))

(fn ConstructionScript)

(fn MappingContextAdd
  (params (MappingContext :type Input%20Mapping%20Context%20Object%20Reference))
  (bind _returnvalue (PlayerController|LocalPlayerSubsystems|GetEnhancedInputLocalPlayerSubsystem))
  (Utilities|IsValid _returnvalue
    (:Is%20Valid
      (Input|AddMappingContext _returnvalue MappingContext 0 "(bIgnoreAllPressedKeysUntilRelease=True,bForceImmediately=False,bNotifyUserSettings=False)"))))

(fn MappingContextRemove
  (params (MappingContext :type Input%20Mapping%20Context%20Object%20Reference))
  (bind _returnvalue (PlayerController|LocalPlayerSubsystems|GetEnhancedInputLocalPlayerSubsystem))
  (Utilities|IsValid _returnvalue
    (:Is%20Valid
      (Input|RemoveMappingContext _returnvalue MappingContext "(bIgnoreAllPressedKeysUntilRelease=True,bForceImmediately=False,bNotifyUserSettings=False)"))))

(fn ShowMouse
  (bind _hud (Variables|Default|GetHUD))
  (if (and (Utilities|Enum|Equal(Enum) (Variables|/Game/Blueprint/Player/BPC_HUD.BPC_HUD_C|GetCurrentController _hud) "NewEnumerator1") (Utilities|Enum|NotEqual(Enum) (Variables|/Game/Blueprint/Player/BPC_HUD.BPC_HUD_C|GetMenu _hud) "NewEnumerator3"))
    (Variables|Default|SetbShowMouseCursor true)
    (else
      (Variables|Default|SetbShowMouseCursor false))))

(fn Back
  (bind _hud (Variables|Default|GetHUD))
  (switch Utilities|FlowControl|Switch|SwitchonE_Menus (Variables|/Game/Blueprint/Player/BPC_HUD.BPC_HUD_C|GetMenu (Variables|Default|GetHUD))
    (:NewEnumerator0
      (Default|ClosePauseMenu _hud))
    (:NewEnumerator1
      (Default|CloseSettings _hud))
    (:NewEnumerator7
      (Default|ConfirmRemove _hud))))

(fn Accept
  (bind _hud (Variables|Default|GetHUD))
  (bind _currentbutton (Variables|/Game/Blueprint/Player/BPC_HUD.BPC_HUD_C|GetCurrentButton _hud))
  (Utilities|IsValid _currentbutton
    (:Is%20Valid
      (Default|OnButtonPressed _currentbutton))))

(fn VerticalMove
  (params (InputValue :type Float%20%28double-precision%29))
  (bind _hud (Variables|Default|GetHUD))
  (bind _hud_2 (Variables|Default|GetHUD))
  (bind _hud_3 (Variables|Default|GetHUD))
  (bind _output_get (LocalVariables|SetValue InputValue))
  (LocalVariables|SetTrue (> _output_get 0.0))
  (switch Utilities|FlowControl|Switch|SwitchonE_Menus (Variables|/Game/Blueprint/Player/BPC_HUD.BPC_HUD_C|GetMenu (Variables|Default|GetHUD))
    (:NewEnumerator2
      (if (LocalVariables|GetTrue)
        (Default|MainMenuUpButton _hud_3)
        (else
          (Default|MainMenuDownButton _hud_3))))
    (:NewEnumerator0
      (if (LocalVariables|GetTrue)
        (Default|PauseUpButton _hud_2)
        (else
          (Default|PauseDownButton _hud_2))))
    (:NewEnumerator1
      (if (LocalVariables|GetTrue)
        (Default|SettingsPreviousElement _hud)
        (else
          (Default|SettingsNextElement _hud))))))

(fn ChangeTab
  (params (InputValue :type Float%20%28double-precision%29))
  (bind _hud (Variables|Default|GetHUD))
  (LocalVariables|SetValue InputValue)
  (switch Utilities|FlowControl|Switch|SwitchonE_Menus (Variables|/Game/Blueprint/Player/BPC_HUD.BPC_HUD_C|GetMenu (Variables|Default|GetHUD))
    (:NewEnumerator1
      (if (> (LocalVariables|GetValue) 0.0)
        (Default|NextTab _hud)
        (else
          (Default|PreviousTab _hud))))))

(fn HorizontalMove
  (params (InputValue :type Float%20%28double-precision%29))
  (bind _hud (Variables|Default|GetHUD))
  (bind _hud_2 (Variables|Default|GetHUD))
  (LocalVariables|SetValue InputValue)
  (switch Utilities|FlowControl|Switch|SwitchonE_Menus (Variables|/Game/Blueprint/Player/BPC_HUD.BPC_HUD_C|GetMenu (Variables|Default|GetHUD))
    (:NewEnumerator1
      (if (> (LocalVariables|GetValue) 0.0)
        (Default|SettingsRightSetting _hud_2)
        (else
          (Default|SettingsLeftSetting _hud_2))))
    (:NewEnumerator7
      (if (> (LocalVariables|GetValue) 0.0)
        (Default|ConfirmRight _hud)
        (else
          (Default|ConfirmLeft _hud))))))

(fn ClosePause
  (switch Utilities|FlowControl|Switch|SwitchonE_Menus (Variables|/Game/Blueprint/Player/BPC_HUD.BPC_HUD_C|GetMenu (Variables|Default|GetHUD))
    (:NewEnumerator0
      (Default|ClosePauseMenu (Variables|Default|GetHUD)))))