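; A destructible level element built on a Chaos Geometry Collection, with the fractured asset set per instance in the construction script.
; Its Explode event fires once, marks the element destroyed and applies a very large impulse along the given forward vector.
; On each Chaos break event, the component switches to world-dynamic collision that ignores pawns and spawns attached wall dust at the break location.
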(event OnChaosBreakEvent(GeometryCollection)
  (params (BreakEvent :type Chaos%20Break%20Event%20Structure%20%28by%20ref%29))
  ;[1 0 0 1 34] Mesh fracture
  (Collision|SetCollisionObjectType (.component BreakEvent) "ECC_WorldDynamic")
  (Collision|SetCollisionResponsetoChannel (.component BreakEvent) "ECC_Pawn" "ECR_Ignore")
  (Niagara|SpawnSystemAttached "/Game/VFX/wall_destruction/N_wall_dust.N_wall_dust" (.component BreakEvent) "None" (.location BreakEvent) "0, 0, 0" "KeepWorldPosition" true))

(event Custom|Explode
  (params (forward :type Vector))
  (bind _geometrycollection (Variables|Default|GetGeometryCollection))
  ;[1 0 0 1 34] Mesh fracture
  (Utilities|FlowControl|DoOnce false
    (:Completed
      (Variables|Default|SethasBeenDestroyed true)
      (Physics|AddImpulseatLocation _geometrycollection (* forward 1e+06) (Transformation|GetWorldLocation _geometrycollection) "None"))))

(fn ConstructionScript
  (Class|GeometryCollectionComponent|SetRestCollection (Variables|Default|GetGeometryCollection) (Variables|Default|GetgeometryToUse) true))