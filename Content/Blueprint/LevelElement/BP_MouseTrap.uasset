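; BP_MouseTrap is a level-element hazard that snaps shut and kills the player who touches it.
; When CanKill is set, a BP_Player overlapping the Box plays a Timeline that lerps the rod, lever and bar meshes toward their closed poses.
; A second track lifts and tilts the trap, and Death is called on the player only when the animation finishes.
; The construction script checks IsUsed but does nothing with it.
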(event OnComponentBeginOverlap(Box)
  (params (OverlappedComponent :type Primitive%20Component%20Object%20Reference) (OtherActor :type Actor%20Object%20Reference) (OtherComp :type Primitive%20Component%20Object%20Reference) (OtherBodyIndex :type Integer) (bFromSweep :type Boolean) (SweepResult :type Hit%20Result%20Structure%20%28by%20ref%29))
  (if (Variables|Default|GetcanKill)
    (bind _asbp_player (Utilities|Casting|CastToBP_Player OtherActor))
    (bind (_direction _alpha _newtrack_1) (Timeline|Timeline PlayFromStart)
      (:Update
        (Transformation|SetRelativeTransform (Variables|Default|GetMouseTrap_Tige) (Math|Transform|MakeTransform (Math|Vector|Lerp(Vector) "-23.000000,-5.400000,-1.700000" (Variables|Default|GetLoc_End_Tige) _alpha) (Math|Rotator|Lerp(Rotator) "-0.600000,21.400000,1.600000" (Variables|Default|GetRot_End_Tige) _alpha) "1.000000,1.000000,1.000000") false false)
        (Transformation|SetRelativeTransform (Variables|Default|GetMouseTrap_Elever) (Math|Transform|MakeTransform "0, 0, 0" (Math|Rotator|Lerp(Rotator) "0.000000,0.000000,-10.000000" "0, 0, 0" _alpha) "1.000000,1.000000,1.000000") false false)
        (Transformation|SetRelativeTransform (Variables|Default|GetMouseTrap_Bare) (Math|Transform|MakeTransform (Math|Vector|Lerp(Vector) "0.000000,0.000000,30.160000" "0, 0, 0" _alpha) (Math|Rotator|Lerp(Rotator) "0.000000,0.000000,183.170000" (Variables|Default|GetRot_End_Bare) _alpha) "1.000000,1.000000,1.000000") false false)
        (Transformation|SetRelativeTransform (Variables|Default|GetMouseTrap) (Math|Transform|MakeTransform (Math|Vector|Lerp(Vector) "0, 0, 0" "0.000000,0.000000,20.000000" _newtrack_1) (Math|Rotator|Lerp(Rotator) "0, 0, 0" "-15.000000,0.000000,0.000000" _newtrack_1) "1.000000,1.000000,1.000000") false false))
      (:Finished
        (Default|Death _asbp_player)))))

(fn ConstructionScript
  (if (Variables|Default|GetisUsed)
    _))