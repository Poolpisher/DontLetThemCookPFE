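; BP_MinionToadTongue is a toad minion Blueprint that stages a tongue visual with a cable.
; Its Tongue event hides the mesh's Tongue bone, reveals the Cable and attaches its end to the Point actor.
; It also spawns a scaled-up frog tongue Niagara effect at a location computed from actor positions.
; The construction script runs the parent's version, then applies the tongue material to the Cable.
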(event Custom|Tongue
  (bind _returnvalue (Transformation|GetActorLocation))
  (bind _returnvalue_2 (Transformation|GetActorLocation))
  (bind _returnvalue_3 (Math|Vector|GetUnitDirection(Vector) _returnvalue_2 _returnvalue))
  (bind _returnvalue_4 (* _returnvalue_3 5e+01))
  (bind _returnvalue_5 (+ _returnvalue_2 _returnvalue_4))
  (Components|SkinnedMesh|HideBonebyName (Variables|Character|GetMesh) "Tongue" "PBO_None")
  (Rendering|SetVisibility (Variables|Default|GetCable) true false)
  (Class|CableComponent|SetAttachEndto (Variables|Default|GetCable) (Variables|Default|GetPoint) "None" "None")
  (Niagara|SpawnSystematLocation "/Game/Maps/GA/VFX/frog_tongue/N_frog_tongue_test.N_frog_tongue_test" (Math|Vector|MakeVector (.x _returnvalue_5) (.y _returnvalue_5) (.Z (Math|Vector|BreakVector _returnvalue_2))) "0, 0, 0" "10.000000,10.000000,10.000000"))

(fn ConstructionScript
  (|CallParentFunction)
  (Rendering|Material|SetMaterial (Variables|Default|GetCable) 0 "/Game/Models/Characters/Frog/Materials/M_Tongue.M_Tongue"))