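; Toad minion that stretches its tongue to a BP_ToadPoint as a rope.
; Interacting toggles between release and walking to the point nearest the player within range, where a timer detects arrival.
; The tongue bone is then hidden and a child-actor BP_Rope attaches with collision enabled.
; ClimbtoPoint lerps the toad to the point by timeline, then releases; Tick faces the point and releases if the player strays too far.
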(event Custom|Grab
  (params (toadPoint :type BP%20Toad%20Point%20Object%20Reference) (Controller :type Controller%20Object%20Reference))
  ;[1 1 0 1 34] Grab and release
  (Variables|Default|SettoadPoint toadPoint)
  (AI|Navigation|SimpleMovetoLocation Controller (Transformation|GetWorldLocation (Variables|/Game/Blueprint/LevelElement/BP_ToadPoint.BP_ToadPoint_C|GetMovePoint toadPoint)))
  (bind _returnvalue (Utilities|Time|SetTimerbyEvent (delegate Custom|CheckIfHasArrived) 0.1 true true))
  (Variables|Default|SetcheckTimer _returnvalue))

(event Custom|Release
  (bind _roperef (Variables|Default|GetropeRef))
  ;[1 1 0 1 34] Grab and release
  (Default|AttachCable (Variables|Default|GetropeRef))
  (Variables|Default|SettoadPoint 0)
  (Components|SkinnedMesh|UnHideBonebyName (Variables|Character|GetMesh) "Tongue")
  (Rendering|SetVisibility (Variables|Default|GetTongue) false false)
  (Variables|/Game/Blueprint/Minions/BP_Rope.BP_Rope_C|SetisActive _roperef false)
  (Default|SetCableCollisions _roperef "NoCollision")
  (Variables|Default|SetisTonguing false))

(event Custom|CheckIfHasArrived
  (bind _returnvalue (Transformation|GetActorLocation))
  (bind _toadpoint (Variables|Default|GettoadPoint))
  (bind _roperef (Variables|Default|GetropeRef))
  (bind _roperef_2 (Variables|Default|GetropeRef))
  (bind _returnvalue_2 (Transformation|GetActorLocation _toadpoint))
  (bind _returnvalue_3 (Math|Vector|GetUnitDirection(Vector) _returnvalue_2 _returnvalue))
  (bind _returnvalue_4 (* _returnvalue_3 5e+01))
  (bind _returnvalue_5 (+ _returnvalue_2 _returnvalue_4))
  ;[1 1 0 1 34] Grab and release
  (if (< (Math|Vector|Distance(Vector) (Transformation|GetActorLocation) (Transformation|GetWorldLocation (Variables|/Game/Blueprint/LevelElement/BP_ToadPoint.BP_ToadPoint_C|GetMovePoint (Variables|Default|GettoadPoint)))) 1e+02)
    (Utilities|Time|ClearandInvalidateTimerbyHandle (Variables|Default|GetcheckTimer))
    (Variables|Default|SetisTonguing true)
    (Utilities|FlowControl|Delay 0.8)
    (Components|SkinnedMesh|HideBonebyName (Variables|Character|GetMesh) "Tongue" "PBO_None")
    (Rendering|SetVisibility (Variables|Default|GetTongue) true false)
    (Default|AttachCable _roperef _toadpoint)
    (Default|SetCableCollisions _roperef "QueryAndPhysics")
    (Variables|/Game/Blueprint/Minions/BP_Rope.BP_Rope_C|SetisActive _roperef_2 true)
    (Default|SetDirection _roperef_2)
    (Niagara|SpawnSystematLocation "/Game/Maps/GA/VFX/frog_tongue/N_frog_tongue.N_frog_tongue" (Math|Vector|MakeVector (.x _returnvalue_5) (.y _returnvalue_5) (.Z (Math|Vector|BreakVector _returnvalue_2))) "0, 0, 0" "10.000000,10.000000,10.000000")))

(event EventBeginPlay
  (bind _tongue (Variables|Default|GetTongue))
  ;[0 0 0 1 34] Start
  (|CallParentFunction)
  (bind _asbp_rope (Utilities|Casting|CastToBP_Rope (Variables|/Script/Engine.ChildActorComponent|GetChildActor _tongue)))
  (bind _output_get (Variables|Default|SetropeRef _asbp_rope))
  (Variables|/Game/Blueprint/Minions/BP_Rope.BP_Rope_C|SetisActive _output_get false)
  (Default|SetCableCollisions _output_get "NoCollision")
  (Rendering|SetVisibility _tongue false false))

(event EventClimbtoPoint
  (params (cable :type BP%20Rope%20Object%20Reference))
  ;[0 1 0 1 34] Climb
  (Variables|Default|SetcurrentBehaviour "NewEnumerator1")
  (if (== (Variables|/Script/Engine.ChildActorComponent|GetChildActor (Variables|Default|GetTongue)) cable)
    (bind _toadpoint (Variables|Default|GettoadPoint)
      (:then
        (bind _output_get (Variables|Default|SetfirstToadLoc (Transformation|GetActorLocation)))
        (bind _track (Timeline|Timeline_Move PlayFromStart)
          (:Update
            (Transformation|SetActorLocation (Math|Vector|Lerp(Vector) _output_get (Transformation|GetActorLocation _toadpoint) _track) false false))
          (:Finished
            (CallFunction|Release)
            (CallFunction|PickDecision "NewEnumerator0"))))
      (:else))))

(event EventTick
  (params (DeltaSeconds :type Float%20%28single-precision%29))
  (bind _returnvalue (Transformation|GetActorRotation))
  ;[0 0 0 1 34] Update
  (|CallParentFunction DeltaSeconds)
  (Variables|Default|GettoadPoint
    (:then
      (Utilities|FlowControl|Sequence
        (:then_0
          (Transformation|SetActorRotation (Math|Rotator|MakeRotator (.roll _returnvalue) (.pitch _returnvalue) (.yaw (Math|Rotator|FindLookatRotation (Transformation|GetActorLocation) (Transformation|GetActorLocation (Variables|Default|GettoadPoint)))))))
        (:then_1
          (if (> (Math|Vector|Distance(Vector) (Transformation|GetActorLocation (Game|GetPlayerCharacter 0)) (Transformation|GetActorLocation)) 1.6e+03)
            ;[0 0 1 1 34] Interact
            (CallFunction|Release)
            (Utilities|Time|PauseTimerbyHandle (Variables|Default|GetcheckTimer))
            (CallFunction|PickDecision "NewEnumerator0")
            (Variables|Default|SetisInteracting false)))))
    (:else)))

(event EventInteract
  ;[0 0 1 1 34] Interact
  (|CallParentFunction)
  (if (Variables|Default|GetisInteracting)
    (CallFunction|Release :!label _label)
    (Utilities|Time|PauseTimerbyHandle (Variables|Default|GetcheckTimer) :!label _label_2)
    (CallFunction|PickDecision "NewEnumerator0")
    (Variables|Default|SetisInteracting false)
    (else
      (bind _outactors (Actor|GetAllActorsOfClass "/Game/Blueprint/LevelElement/BP_ToadPoint.BP_ToadPoint_C"))
      (if (> (Utilities|Array|Length _outactors) 0)
        (bind _toad (CallFunction|GetClosestToadPoint _outactors))
        (Utilities|IsValid _toad
          (:Is%20Valid
            (CallFunction|Grab _toad (Pawn|GetController))
            (Variables|Default|SetisInteracting true))
          (:Is%20Not%20Valid
            (goto _label)))
        (else
          (goto _label_2))))))

(fn ConstructionScript
  (|CallParentFunction)
  (bind _asbp_rope (Utilities|Casting|CastToBP_Rope (Variables|/Script/Engine.ChildActorComponent|GetChildActor (Variables|Default|GetTongue))))
  (Rendering|Material|SetMaterial (Variables|/Game/Blueprint/Minions/BP_Rope.BP_Rope_C|GetCable _asbp_rope) 0 "/Game/Models/Characters/Frog/Materials/M_Tongue.M_Tongue"))

(fn GetClosestToadPoint
  (params (pointsArray :type Array%20of%20BP%20Toad%20Point%20Object%20References))
  (LocalVariables|SetlastDistance 999999999999.0)
  (for _array_element pointsArray
    (if (and (< (Math|Vector|Distance(Vector) (Transformation|GetActorLocation _array_element) (Transformation|GetActorLocation (Game|GetPlayerCharacter 0))) (LocalVariables|GetlastDistance)) (< (Math|Vector|Distance(Vector) (Transformation|GetActorLocation _array_element) (Transformation|GetActorLocation (Game|GetPlayerCharacter 0))) 1.6e+03))
      (LocalVariables|SetlastDistance (Math|Vector|Distance(Vector) (Transformation|GetActorLocation _array_element) (Transformation|GetActorLocation (Game|GetPlayerCharacter 0))))
      (LocalVariables|SetclosestPoint _array_element)))
  (return (LocalVariables|GetclosestPoint)))