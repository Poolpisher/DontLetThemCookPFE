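; BP_SplineCable is a spline-driven cable Blueprint that tiles a mesh along a spline path.
; Its construction script calls UpdateSpline, which derives segment length from the mesh's X bounds and adds spline mesh components at that spacing.
; Each segment takes local positions and tangents from the spline, with tangent size clamped to the segment length.
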(fn ConstructionScript
  (CallFunction|UpdateSpline))

(fn UpdateSpline
  (bind _mesh (Variables|Default|GetMesh))
  (bind _spline (Variables|Default|GetSpline))
  (bind _spline_2 (Variables|Default|GetSpline))
  (bind _returnvalue (StaticMesh|GetBoundingBox _mesh))
  (Variables|Default|SetXLength (.x (+ (Math|Vector|VectorGetAbs (.min _returnvalue)) (Math|Vector|VectorGetAbs (.max _returnvalue)))))
  (for _index (range 0 (Math|Float|Truncate (/ (Spline|GetSplineLength (Variables|Default|GetSpline)) (Variables|Default|GetXLength))))
    (bind _returnvalue_2 (AddComponent|AddSplineMeshComponent false))
    (SplineMesh|SetForwardAxis _returnvalue_2 "X" false)
    (Components|StaticMesh|SetStaticMesh _returnvalue_2 (Variables|Default|GetMesh))
    (SplineMesh|SetStartandEnd _returnvalue_2 (Spline|GetLocationatDistanceAlongSpline _spline_2 (* _index (Variables|Default|GetXLength)) "Local") (Math|Vector|ClampVectorSize (Spline|GetTangentatDistanceAlongSpline _spline_2 (* _index (Variables|Default|GetXLength)) "Local") 0.0 (Variables|Default|GetXLength)) (Spline|GetLocationatDistanceAlongSpline _spline (* (+ _index 1) (Variables|Default|GetXLength)) "Local") (Math|Vector|ClampVectorSize (Spline|GetTangentatDistanceAlongSpline _spline (* (+ _index 1) (Variables|Default|GetXLength)) "Local") 0.0 (Variables|Default|GetXLength)) true :!class /Script/Engine.SplineMeshComponent)))