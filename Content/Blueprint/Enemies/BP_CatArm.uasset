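; BP_CatArm is an enemy cat arm attack that stays hidden from BeginPlay until its Attack event is called.
; Attack reveals the actor and mesh, sets state flags and grows a crack component from zero scale through a timeline.
; After short wind-up delays, a single sphere trace on the Camera channel at the Scene component checks for BP_Player and calls Death on it.
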(event Custom|Attack
  (bind _scene (Variables|Default|GetScene))
  (bind _returnvalue (Transformation|GetWorldLocation _scene))
  ;[1 0 0 1 34] Attack
  (Development|SetHiddeninGame (Variables|Character|GetMesh) true false)
  (Variables|Default|SethasSpawned true)
  (Rendering|SetActorHiddenInGame false)
  (Development|SetHiddeninGame (Variables|Character|GetMesh) false false)
  (CallFunction|SetCrack)
  (Utilities|FlowControl|Delay 0.7)
  (Variables|Default|SetisAttacking true)
  (Utilities|FlowControl|Delay 0.2)
  (bind _outhits (Collision|MultiSphereTraceByChannel _returnvalue _returnvalue 1.5e+02 "TraceTypeQuery2" false 0 "None"))
  (bind _array_element (Utilities|Array|ForEachLoopwithBreak _outhits :!label _label)
    (:LoopBody
      (bind _asbp_player (Utilities|Casting|CastToBP_Player (.HitActor (Collision|BreakHitResult _array_element))))
      (Default|Death _asbp_player)
      (goto _label Break))))

(event Custom|SetCrack
  ;[1 0 0 1 34] Attack
  (bind _track (Timeline|Timeline_Crack PlayFromStart)
    (:Update
      (Transformation|SetWorldScale3D (Variables|Default|GetCrack) (Math|Vector|Lerp(Vector) "0, 0, 0" "4.000000,4.000000,4.000000" _track)))))

(event EventBeginPlay
  ;[0 0 0 1 34] Start
  (Rendering|SetActorHiddenInGame true))

(fn ConstructionScript)