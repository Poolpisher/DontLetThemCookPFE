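; Interactable focus point that flies the view from the player's camera to its Scene transform and opens the W_Book widget with mouse-driven UI input.
; Focus snaps its own camera onto the player's before switching view target, then a timeline lerps location and rotation for the move.
; Interacting again or the player leaving the trigger box reverses the move, removes the widget and restores the player view and game input.
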(event OnComponentEndOverlap(Box)
  (params (OverlappedComponent :type Primitive%20Component%20Object%20Reference) (OtherActor :type Actor%20Object%20Reference) (OtherComp :type Primitive%20Component%20Object%20Reference) (OtherBodyIndex :type Integer))
  ;[1 0 0 1 34] Check trigger exit
  (Utilities|Casting|CastToBP_Player OtherActor)
  (if (Variables|Default|GetisFocused)
    (CallFunction|Unfocus)
    (Variables|Default|SetisFocused false)))

(event Custom|Focus
  (bind _camera (Variables|Default|GetCamera))
  ;[0 1 0 1 34] Focus/Unfocus
  (Variables|Default|SetisFocused true)
  (bind _asbp_player (Utilities|Casting|CastToBP_Player (Game|GetPlayerCharacter 0)))
  (Input|SetInputModeUIOnly (Game|GetPlayerController 0) 0 "DoNotLock" true)
  (Transformation|SetWorldLocationAndRotation _camera (Transformation|GetWorldLocation (Variables|/Game/Blueprint/Camera/BP_Camera.BP_Camera_C|GetCamera (Variables|/Game/Blueprint/Player/BP_Player.BP_Player_C|Getcamera _asbp_player))) (Transformation|GetWorldRotation (Variables|/Game/Blueprint/Camera/BP_Camera.BP_Camera_C|GetCamera (Variables|/Game/Blueprint/Player/BP_Player.BP_Player_C|Getcamera _asbp_player))) false false)
  (Utilities|FlowControl|DelayUntilNextTick)
  (Game|Player|SetViewTargetwithBlend (Game|GetPlayerController 0) (Components|GetOwner _camera) 0.0 "VTBlend_Linear" 0.0 false)
  (Utilities|FlowControl|DelayUntilNextTick)
  (CallFunction|MoveCamera (Variables|Default|GetCamera) (Variables|Default|GetScene))
  (Utilities|FlowControl|Delay 1.0)
  (Variables|/Script/Engine.PlayerController|SetbShowMouseCursor (Game|GetPlayerController 0) true)
  (bind _returnvalue (UserInterface|CreateWidget "/Game/Widgets/W_Book.W_Book_C" 0 self))
  (bind _output_get (Variables|Default|SetbookWidget _returnvalue))
  (UserInterface|Viewport|AddtoViewport _output_get 0))

(event Custom|Unfocus
  (bind _returnvalue (Game|GetPlayerController 0))
  ;[0 1 0 1 34] Focus/Unfocus
  (Variables|Default|SetisFocused false)
  (bind _asbp_player (Utilities|Casting|CastToBP_Player (Game|GetPlayerCharacter 0)))
  (Widget|RemovefromParent (Variables|Default|GetbookWidget))
  (CallFunction|MoveCamera (Variables|Default|GetScene) (Variables|/Game/Blueprint/Camera/BP_Camera.BP_Camera_C|GetCamera (Variables|/Game/Blueprint/Player/BP_Player.BP_Player_C|Getcamera _asbp_player)))
  (Utilities|FlowControl|Delay 1.0)
  (Game|Player|SetViewTargetwithBlend (Game|GetPlayerController 0) (Variables|/Game/Blueprint/Player/BP_Player.BP_Player_C|Getcamera _asbp_player) 0.0 "VTBlend_Linear" 0.0 false)
  (Input|SetInputModeGameOnly _returnvalue true)
  (Variables|/Script/Engine.PlayerController|SetbShowMouseCursor _returnvalue false))

(event Custom|MoveCamera
  (params (firstPos :type Scene%20Component%20Object%20Reference) (target :type Scene%20Component%20Object%20Reference))
  (bind _camera (Variables|Default|GetCamera))
  ;[1 1 0 1 34] Move camera
  (bind _output_get (Variables|Default|SetfirstCamLoc (Transformation|GetWorldLocation firstPos)))
  (bind _output_get_2 (Variables|Default|SetfirstCamRot (Transformation|GetWorldRotation firstPos)))
  (bind _track (Timeline|Timeline PlayFromStart)
    (:Update
      (Transformation|SetWorldLocation _camera (Math|Vector|Lerp(Vector) _output_get (Transformation|GetWorldLocation target) _track) false true)
      (Transformation|SetWorldRotation _camera (Math|Rotator|Lerp(Rotator) _output_get_2 (Transformation|GetWorldRotation target) _track true) false false))))

(event EventInteract
  (params (Interactor :type BPC%20Interactor%20Object%20Reference))
  ;[0 0 1 1 34] Interact
  (if (Variables|Default|GetisFocused)
    (CallFunction|Unfocus)
    (else
      (CallFunction|Focus))))

(fn ConstructionScript)