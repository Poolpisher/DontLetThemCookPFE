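; BP_LobbyLamp is a level-art lamp Blueprint with a configurable spotlight, named for use in a lobby.
; Its construction script copies the Blueprint's variables onto the SpotLight component, covering color, intensity, attenuation, cone angle, source radius, shadow casting and volumetric scattering.
; It has no runtime logic, as the event graph holds only disabled placeholder events.
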(event EventBeginPlay)

(event Collision|EventActorBeginOverlap
  (params (OtherActor :type Actor%20Object%20Reference)))

(event EventTick
  (params (DeltaSeconds :type Float%20%28single-precision%29)))

(fn ConstructionScript
  (bind _spotlight (Variables|Default|GetSpotLight))
  (Rendering|Components|Light|SetLightColor _spotlight (Variables|Default|GetSpotlightColor) true)
  (Rendering|Components|Light|SetIntensity _spotlight (Variables|Default|GetSpotlightIntensity))
  (Rendering|Lighting|SetAttenuationRadius _spotlight (Variables|Default|GetSpotlightAttenuationRadius))
  (Rendering|Lighting|SetOuterConeAngle _spotlight (Variables|Default|GetSpotlightConeAngle))
  (Class|PointLightComponent|SetSourceRadius _spotlight (Variables|Default|GetSpotlightSourceRadius))
  (Rendering|Components|Light|SetCastShadows _spotlight (Variables|Default|GetSpotlightCastShadow))
  (Class|LightComponent|SetVolumetricScatteringIntensity _spotlight (Variables|Default|GetSpotlightVolumetricScattering)))